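; Pickup actor for stone tablet piece A, collected when the main character overlaps its Box.
; The overlap sets the character's tablet flag, unlocks its pause-menu slot and thumbnail, and records tablet A in the game instance.
; It then plays a pickup sound, prints a message and destroys itself; the BP_OpenDoor lookup result goes unused.
; An item popup with movement lock and a CollectItem call are present but unconnected.
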(event `self.Box.OnComponentBeginOverlap`
  (params (OverlappedComponent :type "PrimitiveComponent Object Reference") (OtherActor :type "Actor Object Reference") (OtherComp :type "PrimitiveComponent Object Reference") (OtherBodyIndex :type Integer) (bFromSweep :type Boolean) (SweepResult :type "HitResult Structure (by ref)"))
  (bind _asbp_maincharacter (cast `/Game/Blueprints/BP_Maincharacter` OtherActor))
  (set `/Game/Blueprints/BP_Maincharacter.has tablet` true _asbp_maincharacter)
  (bind _pause_menu_widget (`/Game/Blueprints/BP_Maincharacter.Pause Menu Widget` _asbp_maincharacter))
  (`Widget.SetIsEnabled` (`/Game/Blueprints/UI/WB_PauseMenu.slot3` _pause_menu_widget) true)
  (`Widget.SetVisibility` (`/Game/Blueprints/UI/WB_PauseMenu.TN_tablet_A01` _pause_menu_widget) "SelfHitTestInvisible")
  (bind _asgi_my_game_instance (cast `/Game/Blueprints/GameMode/GI_MyGameInstance` (`GameplayStatics.GetGameInstance`)))
  (set `/Game/Blueprints/GameMode/GI_MyGameInstance.HasTabletA` true _asgi_my_game_instance)
  (`GameplayStatics.GetActorOfClass` "/Game/Blueprints/item/door/BP_OpenDoor.BP_OpenDoor_C")
  (`GameplayStatics.PlaySound2D` "/Game/Audio/Effect/itempicksound.itempicksound" 1.0 1.0 0.0 null null)
  (`KismetSystemLibrary.PrintText` "You got the tablet_A")
  (`self.K2_DestroyActor`))

(fn `UserConstructionScript`)