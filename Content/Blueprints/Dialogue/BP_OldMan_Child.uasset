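; Old man NPC dialogue Blueprint that plays cabin music and a memory video, swapping in Korean lines when set.
; Each Dialogue call halts player movement and advances one line in WB_TalkDialogue, choosing lines from GameInstance progress flags and DialogueIndex.
; The first conversation breaks for the video while music fades out until a delayed fade-in.
; Finishing it unlocks a pause-menu replay button and sets IsTalkWithOldMan.
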(event `self.ReceiveBeginPlay`
  (`|ExecutionSequence`
    (:`then_0`
      ;[1 1 1] Cabin_Bgm
      (bind _returnvalue (`GameplayStatics.SpawnSound2D` "/Game/Audio/RPG_Music_010719/Wavs/WAV_2__Goddess_Ytris.WAV_2__Goddess_Ytris" 1.0 1.0 0.0 null))
      (set `self.CabinBgm` _returnvalue))
    (:`then_1`
      (bind _asgi_my_game_instance (cast `/Game/Blueprints/GameMode/GI_MyGameInstance` (`GameplayStatics.GetGameInstance`)))
      (set `self._GameInstance` _asgi_my_game_instance)
      (bind _asbp_maincharacter (cast `/Game/Blueprints/BP_Maincharacter` (`GameplayStatics.GetPlayerCharacter` 0)))
      (set `self._Player` _asbp_maincharacter)
      (if (`/Game/Blueprints/GameMode/GI_MyGameInstance.bIsKorean` (`self._GameInstance`))
        (set `self.dialogue1` (`self.K_dialogue1`))
        (set `self.dialogue2` (`self.K_dialogue2`))
        (set `self.2ndDialogue_1` (`self.K_2ndDialogue_1`))
        (set `self.2ndDialogue_2` (`self.K_2ndDialogue_2`))
        (set `self.3rdDialogue` (`self.K_3rdDialogue`))))))

(event `/Game/Blueprints/Dialogue/BPI_Dialogue.Dialogue`
  ;[1 1 1] 기본
  (`SceneComponent.SetVisibility` (`self.Widget`) false false)
  (`NavMovementComponent.StopActiveMovement` (`Character.CharacterMovement` (`GameplayStatics.GetPlayerCharacter` 0)))
  (`CharacterMovementComponent.DisableMovement` (`Character.CharacterMovement` (`GameplayStatics.GetPlayerCharacter` 0)))
  (if (`|GetArrayItem` (`/Game/Blueprints/GameMode/GI_MyGameInstance.bIsClear2ndMap_CustomEvent` (`self._GameInstance`)))
    ;[1 1 1] AfterClearPuzzle
    ;;[0.3325 0.3325 0.3325] 1번 대화 - 대화 추가하고 싶으시면 이거 복사해서 숫자 달려있는 변수들 변경해서 쓰십셔
    (`/Engine/EditorBlueprintResources/StandardMacros.IncrementInt` (`self.TalkIndex`)
      (:`  `
        (if (< (`self.TalkIndex`) (`KismetArrayLibrary.Array_Length` (`self.3rdDialogue`)))
          (`self.UI`
            (:`then`
              _)
            (:`else`
              (bind _returnvalue (`|CreateWidget` "/Game/Blueprints/Dialogue/WB_TalkDialogue.WB_TalkDialogue_C" (`GameplayStatics.GetPlayerController` 0)))
              (bind _output_get (set `self.UI` _returnvalue))
              (`UserWidget.AddToViewport` _output_get 0)))
          (`TextBlock.SetText` (`/Game/Blueprints/Dialogue/WB_TalkDialogue.DialogueText` (`self.UI`)) (`KismetTextLibrary.Conv_StringToText` (`|GetArrayItem` (`self.3rdDialogue`) (`self.TalkIndex`))))
          (`GameplayStatics.PlaySound2D` (`self.Sound_1`) 1.0 1.0 0.0 null null)
          (else
            (`self.EndDialogue`)))))
    (elif (`/Game/Blueprints/GameMode/GI_MyGameInstance.bIsTalkWithOldMan` (`self._GameInstance`))
      ;[1 1 1] 기억구슬 획득 전
      (if (== 1 (`self.dialogueIndex`))
        ;;[0.3325 0.3325 0.3325] 1번 대화 - 대화 추가하고 싶으시면 이거 복사해서 숫자 달려있는 변수들 변경해서 쓰십셔
        (`/Engine/EditorBlueprintResources/StandardMacros.IncrementInt` (`self.TalkIndex`)
          (:`  `
            (if (< (`self.TalkIndex`) (`KismetArrayLibrary.Array_Length` (`self.2ndDialogue_1`)))
              (`self.UI`
                (:`then`
                  _)
                (:`else`
                  (bind _returnvalue_2 (`|CreateWidget` "/Game/Blueprints/Dialogue/WB_TalkDialogue.WB_TalkDialogue_C" (`GameplayStatics.GetPlayerController` 0)))
                  (bind _output_get_2 (set `self.UI` _returnvalue_2))
                  (`UserWidget.AddToViewport` _output_get_2 0)))
              (`TextBlock.SetText` (`/Game/Blueprints/Dialogue/WB_TalkDialogue.DialogueText` (`self.UI`)) (`KismetTextLibrary.Conv_StringToText` (`|GetArrayItem` (`self.2ndDialogue_1`) (`self.TalkIndex`))))
              (`GameplayStatics.PlaySound2D` (`self.Sound_1`) 1.0 1.0 0.0 null null)
              (else
                (`self.EndDialogue`)))))
        (elif (== 2 (`self.dialogueIndex`))
          ;;[0.3325 0.3325 0.3325] 2번 대화
          (`/Engine/EditorBlueprintResources/StandardMacros.IncrementInt` (`self.TalkIndex`)
            (:`  `
              (if (< (`self.TalkIndex`) (`KismetArrayLibrary.Array_Length` (`self.2ndDialogue_2`)))
                (`self.UI`
                  (:`then`
                    _)
                  (:`else`
                    (bind _returnvalue_3 (`|CreateWidget` "/Game/Blueprints/Dialogue/WB_TalkDialogue.WB_TalkDialogue_C" (`GameplayStatics.GetPlayerController` 0)))
                    (bind _output_get_3 (set `self.UI` _returnvalue_3))
                    (`UserWidget.AddToViewport` _output_get_3 0)))
                (`TextBlock.SetText` (`/Game/Blueprints/Dialogue/WB_TalkDialogue.DialogueText` (`self.UI`)) (`KismetTextLibrary.Conv_StringToText` (`|GetArrayItem` (`self.2ndDialogue_2`) (`self.TalkIndex`))))
                (`GameplayStatics.PlaySound2D` (`self.Sound_2`) 1.0 1.0 0.0 null null)
                (else
                  (`self.EndDialogue`)))))))
      (else
        ;[1 1 1] First Dialogue - Before Play Video
        (if (`self.IsVideoPlayed`)
          ;;[0.3325 0.3325 0.3325] 2번 대화
          (`/Engine/EditorBlueprintResources/StandardMacros.IncrementInt` (`self.TalkIndex`) :!label _label
            (:`  `
              (if (< (`self.TalkIndex`) (`KismetArrayLibrary.Array_Length` (`self.dialogue2`)))
                (`self.UI`
                  (:`then`
                    _)
                  (:`else`
                    (bind _returnvalue_4 (`|CreateWidget` "/Game/Blueprints/Dialogue/WB_TalkDialogue.WB_TalkDialogue_C" (`GameplayStatics.GetPlayerController` 0)))
                    (bind _output_get_4 (set `self.UI` _returnvalue_4))
                    (`UserWidget.AddToViewport` _output_get_4 0)))
                (`TextBlock.SetText` (`/Game/Blueprints/Dialogue/WB_TalkDialogue.DialogueText` (`self.UI`)) (`KismetTextLibrary.Conv_StringToText` (`|GetArrayItem` (`self.dialogue2`) (`self.TalkIndex`))))
                (`GameplayStatics.PlaySound2D` (`self.Sound_2`) 1.0 1.0 0.0 null null)
                (else
                  (`self.EndDialogue`)
                  ;;[1 1 1] PauseMenu Third Video Open
                  (`Widget.SetVisibility` (`/Game/Blueprints/UI/WB_PauseMenu.PlayButton_3` (`/Game/Blueprints/BP_Maincharacter.Pause Menu Widget` (`self._Player`))) "Visible")
                  (set `/Game/Blueprints/GameMode/GI_MyGameInstance.bIsTalkWithOldMan` true (`self._GameInstance`))))))
          (else
            ;;[0.3325 0.3325 0.3325] 1번 대화 - 대화 추가하고 싶으시면 이거 복사해서 숫자 달려있는 변수들 변경해서 쓰십셔
            (`/Engine/EditorBlueprintResources/StandardMacros.IncrementInt` (`self.TalkIndex`)
              (:`  `
                (if (< (`self.TalkIndex`) (`KismetArrayLibrary.Array_Length` (`self.dialogue1`)))
                  (`self.UI`
                    (:`then`
                      _)
                    (:`else`
                      (bind _returnvalue_5 (`|CreateWidget` "/Game/Blueprints/Dialogue/WB_TalkDialogue.WB_TalkDialogue_C" (`GameplayStatics.GetPlayerController` 0)))
                      (bind _output_get_5 (set `self.UI` _returnvalue_5))
                      (`UserWidget.AddToViewport` _output_get_5 0)))
                  (`TextBlock.SetText` (`/Game/Blueprints/Dialogue/WB_TalkDialogue.DialogueText` (`self.UI`)) (`KismetTextLibrary.Conv_StringToText` (`|GetArrayItem` (`self.dialogue1`) (`self.TalkIndex`))))
                  (`GameplayStatics.PlaySound2D` (`self.Sound_1`) 1.0 1.0 0.0 null null)
                  (else
                    (set `self.TalkIndex` -1)
                    (set `self.dialogueIndex` 2)
                    (`self.DisableInput` (`GameplayStatics.GetPlayerCharacter` 0) (`GameplayStatics.GetPlayerController` 0))
                    (`self.FadeInCabinSound`)
                    ;;[0 1 0.04147] Video
                    (bind _returnvalue_6 (`|CreateWidget` "/Game/Blueprints/transition/WB_LevelTransition.WB_LevelTransition_C"))
                    (`UserWidget.AddToViewport` _returnvalue_6 0)
                    (`/Game/Blueprints/transition/WB_LevelTransition.Play Fade` _returnvalue_6)
                    (`KismetSystemLibrary.Delay` 1.0)
                    (`/Game/Blueprints/transition/WB_LevelTransition.Play Fade Reverse` _returnvalue_6)
                    (bind _returnvalue_7 (`|CreateWidget` "/Game/Blueprints/pachamamaplay/WB_MemoryVideo_A03.WB_MemoryVideo_A03_C"))
                    (`/Game/Blueprints/pachamamaplay/WB_MemoryVideo_A03.Remove video` _returnvalue_7)
                    (`UserWidget.AddToViewport` _returnvalue_7 0)
                    (`KismetSystemLibrary.Delay` 0.2)
                    (set `self.IsVideoPlayed` true)
                    (`self.FadeoutCabinSound`)
                    (`self.EnableInput` (`GameplayStatics.GetPlayerCharacter` 0) (`GameplayStatics.GetPlayerController` 0))
                    (goto _label)))))))))))

(event `FadeInCabinSound`
  ;[1 1 1] bgm fade in
  (`KismetSystemLibrary.Delay` 27.0)
  (`AudioComponent.FadeIn` (`self.CabinBgm`) 1.0 1.0 0.0 "Linear"))

(event `FadeoutCabinSound`
  ;[1 1 1] bgm fade out
  (`AudioComponent.FadeOut` (`self.CabinBgm`) 2.0 0.0 "Linear"))

(fn `UserConstructionScript`
  (`parent.UserConstructionScript`))