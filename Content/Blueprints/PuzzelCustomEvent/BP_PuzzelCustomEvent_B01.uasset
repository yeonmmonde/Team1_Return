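; Puzzle event actor that opens a passage or barrier by lowering its Box component, likely on the main map.
; CustomEvent sets this event's slot in the game instance's main-map cleared-event array, then plays a timeline that lerps the Box down along relative Z.
; AlreadyPlayedEvent snaps the Box straight to the lowered position for an event already played.
; BeginPlay and SolvePuzzel2 are empty.
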(event `self.ReceiveBeginPlay`)

(event `SolvePuzzel2`)

(event `self.CustomEvent`
  (bind _asgi_my_game_instance (cast `/Game/Blueprints/GameMode/GI_MyGameInstance` (`GameplayStatics.GetGameInstance`)))
  (`KismetArrayLibrary.Array_Set` (`/Game/Blueprints/GameMode/GI_MyGameInstance.bIsClearMain_Map_CustomEvent` _asgi_my_game_instance) 1 true)
  (bind (_direction _door) (`Timeline|타임라인`)
    (:`Update`
      (`SceneComponent.K2_SetRelativeLocation` (`self.Box`) (`KismetMathLibrary.MakeVector` 0.0 0.0 (`KismetMathLibrary.Lerp` 0.0 -450.0 _door)) false false))))

(event `self.AlreadyPlayedEvent`
  (`SceneComponent.K2_SetRelativeLocation` (`self.Box`) (0.0 0.0 -450.0) false false))

(fn `UserConstructionScript`)