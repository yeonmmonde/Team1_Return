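; Puzzle event actor that moves three ground pieces and records a main-map custom event as cleared.
; CustomEvent sets index 2 of IsClearMainMapCustomEvent in GI_MyGameInstance, then lerps the pieces' relative locations with three timelines.
; Each timeline starts the next from its Update output, so the movements overlap rather than run sequentially.
; AlreadyPlayedEvent sets fixed relative rotations, not locations, on the pieces; SolvePuzzle3 is empty.
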(event `self.ReceiveBeginPlay`)

(event `SolvePuzzle3`)

(event `self.CustomEvent`
  (bind _asgi_my_game_instance (cast `/Game/Blueprints/GameMode/GI_MyGameInstance` (`GameplayStatics.GetGameInstance`)))
  (`KismetArrayLibrary.Array_Set` (`/Game/Blueprints/GameMode/GI_MyGameInstance.bIsClearMain_Map_CustomEvent` _asgi_my_game_instance) 2 true)
  (bind (_direction `_새_트랙_0`) (`Timeline|타임라인_0`)
    (:`Update`
      (`SceneComponent.K2_SetRelativeLocation` (`self.ground1`) (`KismetMathLibrary.MakeVector` (`KismetMathLibrary.Lerp` -831.143537 -1129.679104 `_새_트랙_0`) (`KismetMathLibrary.Lerp` 498.992807 -192.048179 `_새_트랙_0`)) false false)
      (bind (_direction_2 `_새_트랙_0_2`) (`Timeline|타임라인`)
        (:`Update`
          (`SceneComponent.K2_SetRelativeLocation` (`self.ground2`) (`KismetMathLibrary.MakeVector` (`KismetMathLibrary.Lerp` -1460.354525 -2093.684334 `_새_트랙_0_2`) (`KismetMathLibrary.Lerp` 2052.00971 2048.809479 `_새_트랙_0_2`)) false false)
          (bind (_direction_3 `_새_트랙_0_3`) (`Timeline|타임라인_1`)
            (:`Update`
              (`SceneComponent.K2_SetRelativeLocation` (`self.ground3`) (`KismetMathLibrary.MakeVector` (`KismetMathLibrary.Lerp` 0.0 -3505.861914 `_새_트랙_0_3`) (`KismetMathLibrary.Lerp` 0.0 2320.94272 `_새_트랙_0_3`) (`KismetMathLibrary.Lerp` 0.0 1670.752672 `_새_트랙_0_3`)) false false))))))))

(event `self.AlreadyPlayedEvent`
  (`SceneComponent.K2_SetRelativeRotation` (`self.ground1`) (`KismetMathLibrary.MakeRotator` 455.290494 -311.970983) false false)
  (`SceneComponent.K2_SetRelativeRotation` (`self.ground2`) (`KismetMathLibrary.MakeRotator` 1507.861976 1239.10228) false false)
  (`SceneComponent.K2_SetRelativeRotation` (`self.ground3`) (`KismetMathLibrary.MakeRotator` -1523.501524 -171.259402) false false))

(fn `UserConstructionScript`)