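; BP_BrokenHeart_A01 is a Broken Heart pickup that the main character collects by walking into its box trigger.
; On overlap it sets the HasHeart flag on GI_MyGameInstance, then enables Slot1 and reveals the broken heart element in the character's pause menu widget.
; It then plays a 2D sound, prints a pickup message and destroys itself.
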(event `self.Box.OnComponentBeginOverlap`
  (params (OverlappedComponent :type "PrimitiveComponent Object Reference") (OtherActor :type "Actor Object Reference") (OtherComp :type "PrimitiveComponent Object Reference") (OtherBodyIndex :type Integer) (bFromSweep :type Boolean) (SweepResult :type "HitResult Structure (by ref)"))
  (bind _asbp_maincharacter (cast `/Game/Blueprints/BP_Maincharacter` OtherActor))
  (bind _asgi_my_game_instance (cast `/Game/Blueprints/GameMode/GI_MyGameInstance` (`GameplayStatics.GetGameInstance`)))
  (set `/Game/Blueprints/GameMode/GI_MyGameInstance.HasHeart` true _asgi_my_game_instance)
  (bind _pause_menu_widget (`/Game/Blueprints/BP_Maincharacter.Pause Menu Widget` _asbp_maincharacter))
  (`Widget.SetIsEnabled` (`/Game/Blueprints/UI/WB_PauseMenu.slot1` _pause_menu_widget) true)
  (`Widget.SetVisibility` (`/Game/Blueprints/UI/WB_PauseMenu.TN_BrokenHeart` _pause_menu_widget) "SelfHitTestInvisible")
  (`GameplayStatics.PlaySound2D` "/Engine/EditorSounds/Notifications/CompileSuccess.CompileSuccess" 1.0 1.0 0.0 null null)
  (`KismetSystemLibrary.PrintText` "You got the Heart")
  (`self.K2_DestroyActor`))

(fn `UserConstructionScript`)