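; BP_Harpy is an enemy that wanders, chases the main character and attacks with fireballs.
; Tick runs a state machine (Idle, Move, Chase, Attack, Nothing), with Move turning by a random per-instance yaw step.
; CheckPlayer line-traces for visibility within a distance, selecting attack up close, chase farther out, otherwise wandering.
; Attack faces the player, enters Nothing, plays a montage, spawns BP_FireBall after a delay, then returns to Idle.
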(event `self.ReceiveBeginPlay`
  (bind _returnvalue (`KismetMathLibrary.RandomFloatInRange` -1.0 1.0))
  (set `self.StartPosition` (`self.K2_GetActorLocation`))
  (bind _asbp_maincharacter (cast `/Game/Blueprints/BP_Maincharacter` (`GameplayStatics.GetPlayerCharacter` 0)))
  (set `self.Player` _asbp_maincharacter)
  (if (== _returnvalue 0.0)
    (set `self.RandomPosition` 1.0)
    (else
      (set `self.RandomPosition` _returnvalue))))

(event `self.ReceiveTick`
  (params (DeltaSeconds :type "Float (single-precision)"))
  (bind (_returnvalue_roll _returnvalue_pitch _returnvalue_yaw) (`KismetMathLibrary.BreakRotator` (`self.K2_GetActorRotation`)))
  (bind (_returnvalue_x _returnvalue_y) (`KismetMathLibrary.BreakVector` (- (`self.K2_GetActorLocation` (`self.Player`)) (`self.K2_GetActorLocation`))))
  (set `self.bIsMove` true)
  (switch `/Game/AI/Enemy_JINA/E_HarpyState` (`self.State`)
    (:`NewEnumerator0`
      (`KismetSystemLibrary.Delay` (`KismetMathLibrary.RandomFloatInRange` 0.5 1.5))
      (bind _isfindplayer (`self.Check Player` 2000.0 :!label _label))
      (if _isfindplayer
        (set `self.State` "NewEnumerator3")
        (else
          (bind _isfindplayer_2 (`self.Check Player` 3000.0 :!label _label_2))
          (if _isfindplayer_2
            (set `self.bIsFind` true)
            (set `self.State` "NewEnumerator2")
            (else
              (set `self.State` "NewEnumerator1")
              (set `self.bIsFind` false))))))
    (:`NewEnumerator1`
      (`self.K2_SetActorRotation` (`KismetMathLibrary.MakeRotator` 0.0 0.0 (+ _returnvalue_yaw (`self.RandomPosition`))))
      (`self.AddMovementInput` (`self.GetActorForwardVector`))
      (goto _label_2))
    (:`NewEnumerator2`
      (`self.AddMovementInput` (`KismetMathLibrary.Normal` (`KismetMathLibrary.MakeVector` _returnvalue_x _returnvalue_y)) 0.5)
      (goto _label))
    (:`NewEnumerator3`
      (`self.K2_SetActorRotation` (`KismetMathLibrary.Conv_VectorToRotator` (- (`self.K2_GetActorLocation` (`self.Player`)) (`self.K2_GetActorLocation`))))
      (set `self.State` "NewEnumerator4")
      (`self.PlayAnimMontage` "/Game/AI/Enemy_JINA/Montage_Harpy.Montage_Harpy")
      (`KismetSystemLibrary.Delay` 1.0)
      (`|SpawnActorFromClass` "/Game/AI/Enemy_JINA/BP_FireBall.BP_FireBall_C" (`self.GetTransform`) "Undefined" "MultiplyWithRoot" null null)
      (set `self.State` "NewEnumerator0"))
    (:`NewEnumerator4`
      (set `self.bIsMove` false))))

(fn `Check Player`
  (params (Distance :type "Float (double-precision)"))
  (returns (IsFindPlayer :type Boolean))
  (bind _outhit (`KismetSystemLibrary.LineTraceSingle` (`self.K2_GetActorLocation`) (`self.K2_GetActorLocation` (`self.Player`)) "TraceTypeQuery3"))
  (bind (_bblockinghit _binitialoverlap _time _distance _location _impactpoint _normal _impactnormal _physmat _hitactor) (`GameplayStatics.BreakHitResult` _outhit))
  (if (<= _distance Distance)
    (cast `/Game/Blueprints/BP_Maincharacter` _hitactor
      (:`then`
        (return true))
      (:`CastFailed`
        (return false)))
    (else
      (return false))))

(fn `SetRandomDirection`
  (returns (NewParam :type "Vector Structure"))
  (if (`KismetMathLibrary.RandomBool`)
    (return (1.0 1.0 0.0))
    (else
      (return (1.0 -1.0 0.0)))))

(fn `UserConstructionScript`)