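; BP_OpenDoor is a door actor that slides its mesh upward along Z with a timeline.
; Entering its box shows a prompt, caches the BP_Maincharacter and enables input, so pressing E opens the door after a short delay if HasTablet is set.
; A separate collectitem event counts items and opens the door once the maximum is reached.
; Input stays enabled afterward because the DisableInput call is unconnected.
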(event `Open Door`
  (bind (_direction `_새_트랙_0`) (`Timeline|Open Door Anim`)
    (:`Update`
      (`SceneComponent.K2_SetRelativeLocation` (`self.SM_door_A01`) (`KismetMathLibrary.MakeVector` 0.0 0.0 (`KismetMathLibrary.Lerp` 0.0 388.0 `_새_트랙_0`)) false false))))

(event `Key|E`
  (params (Key :type "Key Structure"))
  (:`Pressed`
    (if (`/Game/Blueprints/BP_Maincharacter.has tablet` (stale `self.Box.OnComponentBeginOverlap` _asbp_maincharacter))
      (`KismetSystemLibrary.Delay` 0.3)
      (`self.Open Door`)
      (else
        (`KismetSystemLibrary.PrintText` "you dont have eye")))))

(event `collect item`
  (`/Engine/EditorBlueprintResources/StandardMacros.IncrementInt` (`self.curruntitemcollected`)
    (:`  `
      (if (>= (`self.curruntitemcollected`) (`self.maxitemcollectable`))
        (`/Engine/EditorBlueprintResources/StandardMacros.DoOnce` false
          (:`Completed`
            (`self.Open Door`)))))))

(event `self.Box.OnComponentBeginOverlap`
  (params (OverlappedComponent :type "PrimitiveComponent Object Reference") (OtherActor :type "Actor Object Reference") (OtherComp :type "PrimitiveComponent Object Reference") (OtherBodyIndex :type Integer) (bFromSweep :type Boolean) (SweepResult :type "HitResult Structure (by ref)"))
  (`KismetSystemLibrary.PrintText` "press E")
  (bind _asbp_maincharacter (cast `/Game/Blueprints/BP_Maincharacter` OtherActor))
  (`self.EnableInput` (`GameplayStatics.GetPlayerController` 0)))

(fn `UserConstructionScript`)