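; Pachamama prayer interaction that grants the player's first memory orb and plays a memory video.
; Overlapping the sphere shows a widget and locks movement; pressing E makes the character pray, spawning particles and revealing the orb.
; A light timeline's Update unlocks a pause-menu button, sets the GameInstance flag and restores movement.
; Its BeginPlay music fades out for the video, returns after a fixed delay, then the actor destroys itself.
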(event `self.ReceiveBeginPlay`
  ;[1 1 1] 코멘트
  (bind _returnvalue (`GameplayStatics.SpawnSound2D` "/Game/Audio/Music/A_Fool_s_Theme_-_Brian_Bolger.A_Fool_s_Theme_-_Brian_Bolger" 1.0 1.0 0.0 null false false))
  (set `self.audio` _returnvalue))

(event `view orb`
  ;[1 1 1] 아이템
  (`SceneComponent.SetVisibility` (`self.Sphere`) true false)
  (`SceneComponent.SetVisibility` (`self.colision`) true false))

(event `sound`
  ;[1 1 1] sound
  (`AudioComponent.FadeOut` (`self.audio`) 1.0 0.0 "Linear")
  (`KismetSystemLibrary.Delay` 84.0)
  (`AudioComponent.FadeIn` (`self.audio`) 1.0 1.0 0.0 "Linear")
  (`KismetSystemLibrary.PrintString` "ssss")
  (`self.K2_DestroyActor`))

(event `Key|E`
  (params (Key :type "Key Structure"))
  ;[1 1 1] 코멘트
  (:`Pressed`
    (bind _output_get (set `self.IsPressE?` true))
    (if _output_get :!label _label
      (`SceneComponent.SetVisibility` (`self.Widget`) false false)
      (`/Game/Blueprints/BP_Maincharacter.pray` (stale `self.Sphere1.OnComponentBeginOverlap` _asbp_maincharacter))
      (`|ExecutionSequence`
        (:`then_0`
          ;[1 1 1] 영상플레이
          (`KismetSystemLibrary.Delay` 3.0)
          (bind _returnvalue (`|CreateWidget` "/Game/Blueprints/pachamamaplay/WB_MemoryVideo_A04.WB_MemoryVideo_A04_C"))
          (`/Game/Blueprints/pachamamaplay/WB_MemoryVideo_A04.Remove video2` _returnvalue)
          (`UserWidget.AddToViewport` _returnvalue 0)
          (`self.sound`))
        (:`then_1`
          (`KismetSystemLibrary.Delay` 1.5)
          (`GameplayStatics.SpawnEmitterAtLocation` "/Game/Effect/InfinityBladeEffects/Effects/FX_Mobile/Misc/P_levelUp_Detail2.P_levelUp_Detail2" (15.0 -600.0 300.0) (struct) (0.5 0.5 0.5))
          (`KismetSystemLibrary.Delay` 1.0)
          (`self.view orb`)
          ;[1 1 1] 빛
          (bind (_direction _light) (`Timeline|lighter`)
            (:`Update`
              (`LightComponent.SetIntensity` (`self.PointLight`) _light)
              (`Widget.SetVisibility` (`/Game/Blueprints/UI/WB_PauseMenu.PlayButton_2` (`/Game/Blueprints/BP_Maincharacter.Pause Menu Widget` (stale `self.Sphere1.OnComponentBeginOverlap` _asbp_maincharacter))) "Visible")
              (bind _asgi_my_game_instance (cast `/Game/Blueprints/GameMode/GI_MyGameInstance` (`GameplayStatics.GetGameInstance`)))
              (set `/Game/Blueprints/GameMode/GI_MyGameInstance.bIsGetMemoryBall_First` true _asgi_my_game_instance)
              (`/Game/Blueprints/BP_Maincharacter.enable movement` (stale `self.Sphere1.OnComponentBeginOverlap` _asbp_maincharacter)))))))))

(event `self.Sphere1.OnComponentBeginOverlap`
  (params (OverlappedComponent :type "PrimitiveComponent Object Reference") (OtherActor :type "Actor Object Reference") (OtherComp :type "PrimitiveComponent Object Reference") (OtherBodyIndex :type Integer) (bFromSweep :type Boolean) (SweepResult :type "HitResult Structure (by ref)"))
  ;[1 1 1] 위젯
  (`SceneComponent.SetVisibility` (`self.Widget`) true false)
  (bind _asbp_maincharacter (cast `/Game/Blueprints/BP_Maincharacter` OtherActor))
  (`/Game/Blueprints/BP_Maincharacter.disable movement` _asbp_maincharacter)
  (`self.EnableInput` (`GameplayStatics.GetPlayerController` 0))
  (goto _label))

(event `self.Sphere1.OnComponentEndOverlap`
  (params (OverlappedComponent :type "PrimitiveComponent Object Reference") (OtherActor :type "Actor Object Reference") (OtherComp :type "PrimitiveComponent Object Reference") (OtherBodyIndex :type Integer))
  ;[1 1 1] 위젯
)

(fn `UserConstructionScript`)