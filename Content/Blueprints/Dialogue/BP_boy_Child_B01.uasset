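; Boy child NPC dialogue Blueprint that shows one of two line sequences in a WB_TalkDialogue widget.
; Each Talk hides its widget, freezes player movement, then shows the active sequence's next line with a sound.
; Sequence 2 finishes through End, which removes the UI, restores walking and advances or wraps DialogueIndex.
; Sequence 1 instead zeroes DialogueIndex and disables input without calling End, leaving movement disabled and the UI up.
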(event `/Game/Blueprints/Dialogue/BPI_Talk.Talk`
  ;[1 1 1] 기본
  (`SceneComponent.SetVisibility` (`self.Widget`) false false)
  (`NavMovementComponent.StopActiveMovement` (`Character.CharacterMovement` (`GameplayStatics.GetPlayerCharacter` 0)))
  (`CharacterMovementComponent.DisableMovement` (`Character.CharacterMovement` (`GameplayStatics.GetPlayerCharacter` 0)))
  ;[1 1 1] 기억구슬 획득 전
  (if (== 1 (`self.dialogueIndex`))
    ;;[0.3325 0.3325 0.3325] 1번 대화 - 대화 추가하고 싶으시면 이거 복사해서 숫자 달려있는 변수들 변경해서 쓰십셔
    (`/Engine/EditorBlueprintResources/StandardMacros.IncrementInt` (`self.TalkIndex`)
      (:`  `
        (if (< (`self.TalkIndex`) (`KismetArrayLibrary.Array_Length` (`self.dialogue1`)))
          (`self.UI`
            (:`then`
              _)
            (:`else`
              (bind _returnvalue (`|CreateWidget` "/Game/Blueprints/Dialogue/WB_TalkDialogue.WB_TalkDialogue_C" (`GameplayStatics.GetPlayerController` 0)))
              (bind _output_get (set `self.UI` _returnvalue))
              (`UserWidget.AddToViewport` _output_get 0)))
          (`TextBlock.SetText` (`/Game/Blueprints/Dialogue/WB_TalkDialogue.DialogueText` (`self.UI`)) (`KismetTextLibrary.Conv_StringToText` (`|GetArrayItem` (`self.dialogue1`) (`self.TalkIndex`))))
          (`GameplayStatics.PlaySound2D` (`self.Sound_1`) 1.0 1.0 0.0 null null)
          (else
            (set `self.TalkIndex` -1)
            (set `self.dialogueIndex` 0)
            (`self.DisableInput` null)))))
    (elif (== 2 (`self.dialogueIndex`))
      ;;[0.3325 0.3325 0.3325] 2번 대화
      (`/Engine/EditorBlueprintResources/StandardMacros.IncrementInt` (`self.TalkIndex`)
        (:`  `
          (if (< (`self.TalkIndex`) (`KismetArrayLibrary.Array_Length` (`self.dialogue2`)))
            (`self.UI`
              (:`then`
                _)
              (:`else`
                (bind _returnvalue_2 (`|CreateWidget` "/Game/Blueprints/Dialogue/WB_TalkDialogue.WB_TalkDialogue_C" (`GameplayStatics.GetPlayerController` 0)))
                (bind _output_get_2 (set `self.UI` _returnvalue_2))
                (`UserWidget.AddToViewport` _output_get_2 0)))
            (`TextBlock.SetText` (`/Game/Blueprints/Dialogue/WB_TalkDialogue.DialogueText` (`self.UI`)) (`KismetTextLibrary.Conv_StringToText` (`|GetArrayItem` (`self.dialogue2`) (`self.TalkIndex`))))
            (`GameplayStatics.PlaySound2D` (`self.Sound_2`) 1.0 1.0 0.0 null null)
            (else
              (`self.End`))))))))

(fn `End`
  ;[1 1 1] 대화 종료
  (`Widget.RemoveFromParent` (`self.UI`))
  (`SceneComponent.SetVisibility` (`self.Widget`) true false)
  (`CharacterMovementComponent.SetMovementMode` (`Character.CharacterMovement` (`GameplayStatics.GetPlayerCharacter` 0)) "MOVE_Walking" 0)
  (set `self.TalkIndex` -1)
  (set `self.UI` null)
  (if (== (`self.dialogueCount`) (`self.dialogueIndex`))
    (set `self.dialogueIndex` 1) ; 첫 번째 대화로 초기화
    (else
      (`/Engine/EditorBlueprintResources/StandardMacros.IncrementInt` (`self.dialogueIndex`)))))

(fn `UserConstructionScript`
  (`parent.UserConstructionScript`))