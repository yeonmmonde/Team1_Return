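; BP_DialogueNPC is an early scaffold for an NPC that the player can talk to, with dialogue state and player-lock helpers.
; Start0rProgressDialogue sets IsTalking and resets DialogueStep on first call, with no progression logic yet.
; LockPlayerAndCamera only disables input, while UnlockPlayerAndCamera runs an empty sequence, leaving its EnableInput call unreachable.
; The event graph is empty, nothing here calls these functions, and no camera logic exists.
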(fn `LockPlayerAndCamera`
  (`InputDeviceLibrary.GetPlayerControllerFromInputDevice` (struct))
  (`self.DisableInput` null))

(fn `Start0rProgressDialogue`
  (if (not (`self.IsTalking`))
    (set `self.IsTalking` true)
    (set `self.DialogueStep` 0)))

(fn `UnlockPlayerAndCamera`
  (`|ExecutionSequence`))

(fn `UserConstructionScript`)