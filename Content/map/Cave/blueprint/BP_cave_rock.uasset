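; Cave set-piece Blueprint with trigger boxes that raise rocks, play sounds and light up decals.
; Three rock triggers freeze BP_Maincharacter, destroy themselves, play an earthquake sound and lift meshes via timeline Lerps; only two re-enable movement after a delay.
; Three decal triggers play sounds and animate emissive on dynamic material instances; another plays only a sound.
; Narration widget code and the middle rock's movement re-enable are disconnected.
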(event `self.ReceiveBeginPlay`)

(event `self.Boxdecal1.OnComponentBeginOverlap`
  (params (OverlappedComponent :type "PrimitiveComponent Object Reference") (OtherActor :type "Actor Object Reference") (OtherComp :type "PrimitiveComponent Object Reference") (OtherBodyIndex :type Integer) (bFromSweep :type Boolean) (SweepResult :type "HitResult Structure (by ref)"))
  ;[0.6159 0.9198 1] 1바위
  (`GameplayStatics.SpawnSound2D` "/Game/map/Cave/blueprint/NoOneWillKnow.NoOneWillKnow" 1.0 1.0 0.0 null)
  (bind _returnvalue (`DecalComponent.CreateDynamicMaterialInstance` (`self.Decal_2`)))
  (bind (_direction _emissivevalue) (`Timeline|타임라인_0`)
    (:`Update`
      (`MaterialInstanceDynamic.SetScalarParameterValue` _returnvalue "emessive" _emissivevalue))))

(event `self.Boxdecal.OnComponentBeginOverlap`
  (params (OverlappedComponent :type "PrimitiveComponent Object Reference") (OtherActor :type "Actor Object Reference") (OtherComp :type "PrimitiveComponent Object Reference") (OtherBodyIndex :type Integer) (bFromSweep :type Boolean) (SweepResult :type "HitResult Structure (by ref)"))
  ;[0.6159 0.9198 1] 1바위
  ;;[1 1 1] 데칼
  (`GameplayStatics.SpawnSound2D` "/Game/map/Cave/blueprint/IMadeIt.IMadeIt" 1.0 1.0 0.0 null)
  (bind _returnvalue (`DecalComponent.CreateDynamicMaterialInstance` (`self.Decal_1`)))
  (bind (_direction _emissivevalue) (`Timeline|emmsiveincreased`)
    (:`Update`
      (`MaterialInstanceDynamic.SetScalarParameterValue` _returnvalue "emessive" _emissivevalue))))

(event `self.Boxdecal2.OnComponentBeginOverlap`
  (params (OverlappedComponent :type "PrimitiveComponent Object Reference") (OtherActor :type "Actor Object Reference") (OtherComp :type "PrimitiveComponent Object Reference") (OtherBodyIndex :type Integer) (bFromSweep :type Boolean) (SweepResult :type "HitResult Structure (by ref)"))
  ;[0.6159 0.9198 1] 1바위
  (`GameplayStatics.SpawnSound2D` "/Game/map/Cave/blueprint/WithThisHeart.WithThisHeart" 1.0 1.0 0.0 null)
  (bind _returnvalue (`DecalComponent.CreateDynamicMaterialInstance` (`self.Decal_3`)))
  (bind (_direction _emissivevalue) (`Timeline|타임라인_2`)
    (:`Update`
      (`MaterialInstanceDynamic.SetScalarParameterValue` _returnvalue "emessive" _emissivevalue))))

(event `self.Boxnext.OnComponentBeginOverlap`
  (params (OverlappedComponent :type "PrimitiveComponent Object Reference") (OtherActor :type "Actor Object Reference") (OtherComp :type "PrimitiveComponent Object Reference") (OtherBodyIndex :type Integer) (bFromSweep :type Boolean) (SweepResult :type "HitResult Structure (by ref)"))
  ;[0.6159 0.9198 1] 1바위
  ;;[1 1 1] 바위
  (bind _asbp_maincharacter (cast `/Game/Blueprints/BP_Maincharacter` OtherActor))
  (bind _output_get (set `self.As BP Maincharacter` _asbp_maincharacter))
  (`/Game/Blueprints/BP_Maincharacter.disable movement` _output_get)
  (`KismetSystemLibrary.Delay` 0.3)
  (`ActorComponent.K2_DestroyComponent` (`self.Boxnext`))
  (`GameplayStatics.SpawnSound2D` "/Game/Audio/Effect/wav_earthquake.wav_earthquake" 1.0 1.0 0.0 null)
  (bind (_direction _rockup) (`Timeline|nextrock`)
    (:`Update`
      (`SceneComponent.K2_SetRelativeLocation` (`self.StaticMesh3`) (`KismetMathLibrary.MakeVector` -184.217877 -723.954454 (`KismetMathLibrary.Lerp` -1100.0 0.0 _rockup)) false false)
      (`KismetSystemLibrary.Delay` 5.0)
      (bind _output_get_2 (set `self.As BP Maincharacter` _asbp_maincharacter))
      (`/Game/Blueprints/BP_Maincharacter.enable movement` _output_get_2))))

(event `self.Box1.OnComponentBeginOverlap`
  (params (OverlappedComponent :type "PrimitiveComponent Object Reference") (OtherActor :type "Actor Object Reference") (OtherComp :type "PrimitiveComponent Object Reference") (OtherBodyIndex :type Integer) (bFromSweep :type Boolean) (SweepResult :type "HitResult Structure (by ref)"))
  (bind _asbp_maincharacter (cast `/Game/Blueprints/BP_Maincharacter` OtherActor))
  (bind _output_get (set `self.As BP Maincharacter` _asbp_maincharacter))
  (`/Game/Blueprints/BP_Maincharacter.disable movement` _output_get)
  (`KismetSystemLibrary.Delay` 0.3)
  (`ActorComponent.K2_DestroyComponent` (`self.Box1`))
  (`GameplayStatics.SpawnSound2D` "/Game/Audio/Effect/wav_earthquake.wav_earthquake" 1.0 1.0 0.0 null)
  (bind (_direction _rockup) (`Timeline|타임라인`)
    (:`Update`
      (`SceneComponent.K2_SetRelativeLocation` (`self.StaticMesh6`) (`KismetMathLibrary.MakeVector` -316.602365 -1961.362801 (`KismetMathLibrary.Lerp` -819.163464 0.0 _rockup)) false false))))

(event `self.Box3.OnComponentBeginOverlap`
  (params (OverlappedComponent :type "PrimitiveComponent Object Reference") (OtherActor :type "Actor Object Reference") (OtherComp :type "PrimitiveComponent Object Reference") (OtherBodyIndex :type Integer) (bFromSweep :type Boolean) (SweepResult :type "HitResult Structure (by ref)"))
  (bind _asbp_maincharacter (cast `/Game/Blueprints/BP_Maincharacter` OtherActor))
  (bind _output_get (set `self.As BP Maincharacter` _asbp_maincharacter))
  (`/Game/Blueprints/BP_Maincharacter.disable movement` _output_get)
  (`KismetSystemLibrary.Delay` 0.3)
  (`ActorComponent.K2_DestroyComponent` (`self.Box3`))
  (`GameplayStatics.SpawnSound2D` "/Game/Audio/Effect/wav_earthquake.wav_earthquake" 1.0 1.0 0.0 null)
  (bind (_direction _rockup) (`Timeline|타임라인_1`)
    (:`Update`
      (`SceneComponent.K2_SetRelativeLocation` (`self.StaticMesh10`) (`KismetMathLibrary.MakeVector` -549.924274 -2911.275182 (`KismetMathLibrary.Lerp` -1580.0 0.0 _rockup)) false false)
      (`KismetSystemLibrary.Delay` 5.0)
      (bind _output_get_2 (set `self.As BP Maincharacter` _asbp_maincharacter))
      (`/Game/Blueprints/BP_Maincharacter.enable movement` _output_get_2))))

(event `self.Box.OnComponentBeginOverlap`
  (params (OverlappedComponent :type "PrimitiveComponent Object Reference") (OtherActor :type "Actor Object Reference") (OtherComp :type "PrimitiveComponent Object Reference") (OtherBodyIndex :type Integer) (bFromSweep :type Boolean) (SweepResult :type "HitResult Structure (by ref)"))
  ;[1 1 1] 여기에 음성
  (`GameplayStatics.SpawnSound2D` "/Game/map/Cave/blueprint/NoTimeToWaste.NoTimeToWaste" 1.0 1.0 0.0 null))

(fn `UserConstructionScript`)