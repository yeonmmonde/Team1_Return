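; Puzzle event actor that opens a door in what appears to be the second map by raising its Cube.
; CustomEvent waits briefly, then starts a timeline that lifts the Cube and disables Box collision, while marking the event cleared in GI_MyGameInstance and playing an earthquake sound.
; AlreadyPlayedEvent snaps straight to the open, non-colliding state without animation or sound.
; Both events have no callers within this Blueprint.
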(event `self.CustomEvent`
  (`KismetSystemLibrary.Delay` 3.0)
  (`|ExecutionSequence`
    (:`then_0`
      (bind (_direction _door) (`Timeline|타임라인`)
        (:`Update`
          (`SceneComponent.K2_SetRelativeLocation` (`self.Cube`) (`KismetMathLibrary.MakeVector` 0.0 0.0 (`KismetMathLibrary.Lerp` 0.0 700.0 _door)) false false)
          (`PrimitiveComponent.SetCollisionEnabled` (`self.Box`) "NoCollision"))))
    (:`then_1`
      (bind _asgi_my_game_instance (cast `/Game/Blueprints/GameMode/GI_MyGameInstance` (`GameplayStatics.GetGameInstance`)))
      (`KismetArrayLibrary.Array_Set` (`/Game/Blueprints/GameMode/GI_MyGameInstance.bIsClear2ndMap_CustomEvent` _asgi_my_game_instance) 0 true)
      (`GameplayStatics.SpawnSound2D` "/Game/Audio/Effect/wav_earthquake.wav_earthquake" 1.0 1.0 0.0 null))))

(event `self.AlreadyPlayedEvent`
  (`SceneComponent.K2_SetRelativeLocation` (`self.Cube`) (0.0 0.0 700.0) false false)
  (`PrimitiveComponent.SetCollisionEnabled` (`self.Box`) "NoCollision"))

(fn `UserConstructionScript`)