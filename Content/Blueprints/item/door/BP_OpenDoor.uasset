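; BP_OpenDoor is a door that opens once the player holds both tablets, tracked as HasTabletA and HasTabletB on the game instance.
; Box overlap shows a prompt widget, enables input for the main character and runs the tablet check immediately, as does pressing E.
; On success it clears both flags, reveals two table components with pickup sounds, then raises the door by timeline with a fading sound.
; Input is never disabled on exit, and the item-counter path is unwired.
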(event `Open Door`
  ;[1 1 1] 타블렛
  (`|ExecutionSequence`
    (:`then_0`
      (`KismetSystemLibrary.Delay` 0.5)
      (`SceneComponent.SetVisibility` (`self.table1`) true false)
      (`GameplayStatics.SpawnSound2D` "/Game/Audio/ItemPickup/Item_Pickup.Item_Pickup" 1.0 1.0 0.0 null)
      (`KismetSystemLibrary.Delay` 0.5)
      (`SceneComponent.SetVisibility` (`self.table2`) true false)
      (`GameplayStatics.SpawnSound2D` "/Game/Audio/ItemPickup/Item_Pickup.Item_Pickup" 1.0 1.0 0.0 null)
      ;[1 1 1] 오픈도어
      (bind (_direction `_새_트랙_0`) (`Timeline|Open Door Anim`)
        (:`Update`
          (`SceneComponent.K2_SetRelativeLocation` (`self.SM_door_A01`) (`KismetMathLibrary.MakeVector` 0.0 0.0 (`KismetMathLibrary.Lerp` 0.0 388.0 `_새_트랙_0`)) false false))))
    (:`then_1`
      (`KismetSystemLibrary.Delay` 1.0)
      (bind _returnvalue (`GameplayStatics.SpawnSound2D` "/Game/Audio/Effect/243699__ertfelda__hidden-wall-opening.243699__ertfelda__hidden-wall-opening" 1.0 1.0 0.0 null))
      (bind _output_get (set `self.doorsound` _returnvalue))
      (`KismetSystemLibrary.Delay` 3.0)
      (`AudioComponent.FadeOut` _output_get 1.0 0.0 "Linear"))))

(event `self.ReceiveBeginPlay`)

(event `Key|E`
  (params (Key :type "Key Structure"))
  (:`Pressed`
    (if (`/Game/Blueprints/GameMode/GI_MyGameInstance.HasTabletA` (stale `self.Box.OnComponentBeginOverlap` _asgi_my_game_instance)) :!label _label
      (if (`/Game/Blueprints/GameMode/GI_MyGameInstance.HasTabletB` (stale `self.Box.OnComponentBeginOverlap` _asgi_my_game_instance))
        (`KismetSystemLibrary.Delay` 0.3)
        (`self.Open Door`)
        (set `/Game/Blueprints/GameMode/GI_MyGameInstance.HasTabletA` false (stale `self.Box.OnComponentBeginOverlap` _asgi_my_game_instance))
        (set `/Game/Blueprints/GameMode/GI_MyGameInstance.HasTabletB` false (stale `self.Box.OnComponentBeginOverlap` _asgi_my_game_instance))
        (else
          (`KismetSystemLibrary.PrintText` "you dont have eye2")))
      (else
        (`KismetSystemLibrary.PrintText` "you dont have eye1")))))

(event `self.Box.OnComponentBeginOverlap`
  (params (OverlappedComponent :type "PrimitiveComponent Object Reference") (OtherActor :type "Actor Object Reference") (OtherComp :type "PrimitiveComponent Object Reference") (OtherBodyIndex :type Integer) (bFromSweep :type Boolean) (SweepResult :type "HitResult Structure (by ref)"))
  (`SceneComponent.SetVisibility` (`self.Widget`) true false)
  (`KismetSystemLibrary.PrintText` "press E")
  (cast `/Game/Blueprints/BP_Maincharacter` OtherActor)
  (`self.EnableInput` (`GameplayStatics.GetPlayerController` 0))
  (bind _asgi_my_game_instance (cast `/Game/Blueprints/GameMode/GI_MyGameInstance` (`GameplayStatics.GetGameInstance`)))
  (goto _label))

(event `collect item`)

(event `self.Box.OnComponentEndOverlap`
  (params (OverlappedComponent :type "PrimitiveComponent Object Reference") (OtherActor :type "Actor Object Reference") (OtherComp :type "PrimitiveComponent Object Reference") (OtherBodyIndex :type Integer))
  ;[1 1 1] 오버랩 안됐을때
  (`SceneComponent.SetVisibility` (`self.Widget`) false false))

(fn `UserConstructionScript`)