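; BP_Sensor_Bar is a bar-style sensor that detects the player and can be switched on and off.
; Overlaps on its Trigger pass the other actor to DetectPlayer, which is not defined in this graph.
; Interact flips Activated, toggling both the actor's collision and the visibility of Bars and its children, so a deactivated sensor is hidden and has no collision.
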(event `self.Trigger.OnComponentBeginOverlap`
  (params (OverlappedComponent :type "PrimitiveComponent Object Reference") (OtherActor :type "Actor Object Reference") (OtherComp :type "PrimitiveComponent Object Reference") (OtherBodyIndex :type Integer) (bFromSweep :type Boolean) (SweepResult :type "HitResult Structure (by ref)"))
  (`self.Detect Player` OtherActor))

(event `/Game/Blueprints/BPI_Interact.Interact`
  (if (not (`self.activated`))
    (`self.SetActorEnableCollision` true)
    (`SceneComponent.SetVisibility` (`self.Bars`) true true)
    (set `self.activated` true)
    (else
      (`self.SetActorEnableCollision` false)
      (`SceneComponent.SetVisibility` (`self.Bars`) false true)
      (set `self.activated` false))))

(fn `UserConstructionScript`
  (`parent.UserConstructionScript`))