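; BP_Alarm is an alarm actor that raises a stealth alert across the level.
; StartAlarm plays the alarm sound at its location once until stopped, then calls AlertGuards; StopAlarm fades the sound out and clears the active flag.
; AlertGuards sets hasSeenPlayer on the blackboard of every BP_Guard's AI controller and tells GM_StealthGameMode to switch to escape music.
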(event `Start Alarm`
  (if (not (`self.Alarm Active`))
    (bind _returnvalue (`GameplayStatics.SpawnSoundAtLocation` "/Game/Audio/Alarms/MS_Alarm.MS_Alarm" (`self.K2_GetActorLocation`) (struct) 1.0 1.0 0.0 null null))
    (set `self.Alarm Sound` _returnvalue)
    (set `self.Alarm Active` true)
    (`self.Alert Guards`)))

(event `Stop Alarm`
  (if (`self.Alarm Active`)
    (`AudioComponent.FadeOut` (`self.Alarm Sound`) 0.0 0.0 "Linear")
    (set `self.Alarm Active` false)))

(event `Alert Guards`
  (bind _outactors (`GameplayStatics.GetAllActorsOfClass` "/Game/AI/BP_Guard.BP_Guard_C"))
  (for _array_element _outactors
    (bind _asbp_ai_guard (cast `/Game/AI/BP_AI_Guard` (`AIBlueprintHelperLibrary.GetAIController` _array_element)))
    (`BlackboardComponent.SetValueAsBool` (`AIBlueprintHelperLibrary.GetBlackboard` _asbp_ai_guard) "hasSeenPlayer" true))
  (bind _asgm_stealth_game_mode (cast `/Game/Blueprints/GameMode/GM_StealthGameMode` (`GameplayStatics.GetGameMode`)))
  (`/Game/Blueprints/GameMode/GM_StealthGameMode.Switch Music to Escaping` _asgm_stealth_game_mode))

(fn `UserConstructionScript`)