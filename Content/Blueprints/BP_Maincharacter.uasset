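; Player character Blueprint handling movement, jump, montage dodge roll, crawl and pause menu through Enhanced Input.
; SunGod_Map and Cabin_Map switch to level cameras and add movement input relative to them.
; Crawl lowers walk speed and lengthens the spring arm by timeline; its uncrouch obstacle trace is never called here.
; E triggers BPI_Talk on overlapping NPCs, and custom events handle ragdoll, jewel equipping and return to PlayerStart.
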(event `EnhancedInput|/Game/Blueprints/Input/IA_Move`
  (params (ActionValue :type "Vector2D Structure") (ElapsedSeconds :type "Float (double-precision)") (TriggeredSeconds :type "Float (double-precision)") (InputAction :type "InputAction Object Reference" :default "/Game/Blueprints/Input/IA_Move.IA_Move"))
  ;[1 1 1] Input and Movement
  (:`Triggered`
    (`self.AddMovementInput` (`KismetMathLibrary.GetRightVector` (`self.GetControlRotation`)) ActionValue_X)
    (`self.AddMovementInput` (`KismetMathLibrary.GetForwardVector` (`self.GetControlRotation`)) ActionValue_Y)))

(event `EnhancedInput|/Game/Blueprints/Input/IA_Look`
  (params (ActionValue :type "Vector2D Structure") (ElapsedSeconds :type "Float (double-precision)") (TriggeredSeconds :type "Float (double-precision)") (InputAction :type "InputAction Object Reference" :default "/Game/Blueprints/Input/IA_Look.IA_Look"))
  ;[1 1 1] Input and Movement
  (:`Triggered`
    (`self.AddControllerYawInput` ActionValue_X)
    (`self.AddControllerPitchInput` (* ActionValue_Y -1.0))))

(event `self.ReceiveBeginPlay`
  ;[1 1 1] Input and Movement
  (`|ExecutionSequence`
    (:`then_0`
      (`EnhancedInputSubsystemInterface.AddMappingContext` (pcsubsystem `EnhancedInputLocalPlayerSubsystem` (`GameplayStatics.GetPlayerController` 0)) "/Game/Blueprints/Input/IMC_PlayerInput.IMC_PlayerInput" 0 (struct))
      (bind _returnvalue (`GameplayStatics.GetCurrentLevelName` true))
      (if (`KismetStringLibrary.NotEqual_StrStr` _returnvalue "MainMenu")
        _))
    (:`then_1`
      ;;[1 1 1] SunGod_Map Camera
      (bind _returnvalue_2 (`GameplayStatics.GetCurrentLevelName` true))
      (if (`KismetStringLibrary.EqualEqual_StrStr` _returnvalue_2 "SunGod_Map")
        (`PlayerController.SetViewTargetWithBlend` (`GameplayStatics.GetPlayerController` 0) (`self.SunGodCamera`) 0.0 "VTBlend_Linear" 0.0 false)))
    (:`then_2`
      ;;[1 1 1] Cabin_Map Camera
      (bind _returnvalue_3 (`GameplayStatics.GetCurrentLevelName` true))
      (if (`KismetStringLibrary.EqualEqual_StrStr` _returnvalue_3 "Cabin_Map")
        (`PlayerController.SetViewTargetWithBlend` (`GameplayStatics.GetPlayerController` 0) (`self.CabinCamera`) 0.0 "VTBlend_Linear" 0.0 false)))))

(event `EnhancedInput|/Game/Blueprints/Input/IA_Move`
  (params (ActionValue :type "Vector2D Structure") (ElapsedSeconds :type "Float (double-precision)") (TriggeredSeconds :type "Float (double-precision)") (InputAction :type "InputAction Object Reference" :default "/Game/Blueprints/Input/IA_Move.IA_Move"))
  ;[1 1 1] Input and Movement
  ;;[1 1 1] SunGod_Map Camera
  (:`Triggered`
    (bind _returnvalue (`GameplayStatics.GetCurrentLevelName` true))
    (if (`KismetStringLibrary.EqualEqual_StrStr` _returnvalue "SunGod_Map")
      (`self.AddMovementInput` (`KismetMathLibrary.GetRightVector` (`KismetMathLibrary.ComposeRotators` (`self.GetControlRotation`) (`self.K2_GetActorRotation` (`self.SunGodCamera`)))) ActionValue_X)
      (`self.AddMovementInput` (`KismetMathLibrary.GetForwardVector` (`KismetMathLibrary.ComposeRotators` (`self.GetControlRotation`) (`self.K2_GetActorRotation` (`self.SunGodCamera`)))) ActionValue_Y))))

(event `EnhancedInput|/Game/Blueprints/Input/IA_Move`
  (params (ActionValue :type "Vector2D Structure") (ElapsedSeconds :type "Float (double-precision)") (TriggeredSeconds :type "Float (double-precision)") (InputAction :type "InputAction Object Reference" :default "/Game/Blueprints/Input/IA_Move.IA_Move"))
  ;[1 1 1] Input and Movement
  ;;[1 1 1] Cabin_Map Camera
  (:`Triggered`
    (bind _returnvalue (`GameplayStatics.GetCurrentLevelName` true))
    (if (`KismetStringLibrary.EqualEqual_StrStr` _returnvalue "Cabin_Map")
      (`self.AddMovementInput` (`KismetMathLibrary.GetRightVector` (`KismetMathLibrary.ComposeRotators` (`self.GetControlRotation`) (`self.K2_GetActorRotation` (`self.CabinCamera`)))) ActionValue_X)
      (`self.AddMovementInput` (`KismetMathLibrary.GetForwardVector` (`KismetMathLibrary.ComposeRotators` (`self.GetControlRotation`) (`self.K2_GetActorRotation` (`self.CabinCamera`)))) ActionValue_Y))))

(event `InputAction|IA_JumpFromSetting`
  (params (Key :type "Key Structure"))
  (:`Pressed`
    (if (`self.IsJumping?`)
      _
      (elif (not (`self.IsCrawled?`))
        (`self.Jump`)
        (set `self.IsJumping?` true)
        (if (== (`self.JumpCurrentCount`) 1)
          (`NiagaraFunctionLibrary.SpawnSystemAtLocation` "/Game/Effect/NS_HoldJump.NS_HoldJump" (- (`self.K2_GetActorLocation`) (0.0 0.0 90.0)))))))
  (:`Released`
    (`self.StopJumping`)))

(event `EnhancedInput|/Game/Blueprints/Input/IA_Roll`
  (params (ActionValue :type Boolean) (ElapsedSeconds :type "Float (double-precision)") (TriggeredSeconds :type "Float (double-precision)") (InputAction :type "InputAction Object Reference" :default "/Game/Blueprints/Input/IA_Roll.IA_Roll"))
  ;[1 1 1] Dodge Roll
  (:`Triggered`
    (if (not (`self.is dodging?`))
      (`|PlayMontage` (`self.Mesh`) "/Game/Characters/Robber/Roll/Roll_Montage.Roll_Montage"
        (:`then`
          (set `self.is dodging?` true))
        (:`OnCompleted`
          (set `self.is dodging?` false))))))

(event `EnhancedInput|/Game/Blueprints/Input/IA_Crawl`
  (params (ActionValue :type Boolean) (ElapsedSeconds :type "Float (double-precision)") (TriggeredSeconds :type "Float (double-precision)") (InputAction :type "InputAction Object Reference" :default "/Game/Blueprints/Input/IA_Crawl.IA_Crawl"))
  ;[1 1 1] Crawl
  (:`Started`
    (if (not (`self.IsCrawled?`))
      (set `self.IsCrawled?` true)
      (set `CharacterMovementComponent.MaxWalkSpeed` 150.0 (`self.CharacterMovement`))
      (bind (_direction _arm_length) (`Timeline|Crawl Zoom Out` :!label _label)
        (:`Update`
          (set `SpringArmComponent.TargetArmLength` (`KismetMathLibrary.Lerp` 600.0 750.0 _arm_length) (`self.SpringArm`))))
      (else
        (set `self.IsCrawled?` false)
        (set `CharacterMovementComponent.MaxWalkSpeed` 600.0 (`self.CharacterMovement`))
        (goto _label :!via `Reverse`)))))

(event `Ragdoll`
  (`PrimitiveComponent.SetSimulatePhysics` (`self.Mesh`) true)
  (`self.DisableInput` null))

(event `EnhancedInput|/Game/Blueprints/Input/IA_Pause`
  (params (ActionValue :type Boolean) (ElapsedSeconds :type "Float (double-precision)") (TriggeredSeconds :type "Float (double-precision)") (InputAction :type "InputAction Object Reference" :default "/Game/Blueprints/Input/IA_Pause.IA_Pause"))
  (bind _returnvalue (`GameplayStatics.GetPlayerController` 0))
  (bind _returnvalue_2 (`GameplayStatics.GetPlayerController` 0))
  (:`Started`
    (if (not (`self.paused?`))
      (set `self.paused?` true)
      (bind _returnvalue_3 (`|CreateWidget` "/Game/Blueprints/UI/WB_PauseMenu.WB_PauseMenu_C"))
      (bind _output_get (set `self.Pause Menu Widget` _returnvalue_3))
      (`UserWidget.AddToViewport` _output_get 0)
      (set `PlayerController.bShowMouseCursor` true _returnvalue_2)
      (`WidgetBlueprintLibrary.SetInputMode_GameAndUIEx` _returnvalue_2 (`self.Pause Menu Widget`))
      (`GameplayStatics.SetGamePaused` true)
      (else
        (bind _pause_menu_widget (`self.Pause Menu Widget` :!label _label_2)
          (:`then`
            (`Widget.RemoveFromParent` _pause_menu_widget)
            (set `self.Pause Menu Widget` null)
            (set `self.paused?` false)
            (set `PlayerController.bShowMouseCursor` false _returnvalue)
            (`WidgetBlueprintLibrary.SetInputMode_GameOnly` _returnvalue)
            (`GameplayStatics.SetGamePaused` false))
          (:`else`))))))

(event `Resume`
  (goto _label_2))

(event `Equip Jewel`
  (`SceneComponent.SetVisibility` (`self.Jewel`) true false)
  (set `self.hasJewel` true))

(event `Go To Start`
  (bind _returnvalue (`GameplayStatics.GetActorOfClass` "/Script/Engine.PlayerStart"))
  (`self.K2_SetActorLocation` (`self.K2_GetActorLocation` _returnvalue)))

(event `Key|E`
  (params (Key :type "Key Structure"))
  ;[1 1 1] YoungLady Talk
  (:`Pressed`
    (for _array_element (`self.GetOverlappingActors` "/Game/Blueprints/Dialogue/BP_YoungLady.BP_YoungLady_C")
      (if (`KismetSystemLibrary.DoesImplementInterface` _array_element "/Game/Blueprints/Dialogue/BPI_Talk.BPI_Talk_C")
        (message `/Game/Blueprints/Dialogue/BPI_Talk.Talk` _array_element)))))

(event `Key|E`
  (params (Key :type "Key Structure"))
  ;[1 1 1] YoungMan Talk
  (:`Pressed`
    (for _array_element (`self.GetOverlappingActors` "/Game/Blueprints/Dialogue/BP_YoungMen.BP_YoungMen_C")
      (if (`KismetSystemLibrary.DoesImplementInterface` _array_element "/Game/Blueprints/Dialogue/BPI_Talk.BPI_Talk_C")
        (message `/Game/Blueprints/Dialogue/BPI_Talk.Talk` _array_element)))))

(event `Key|E`
  (params (Key :type "Key Structure"))
  ;[1 1 1] Girl Talk
  (:`Pressed`
    (for _array_element (`self.GetOverlappingActors` "/Game/Blueprints/Dialogue/BP_Girl.BP_Girl_C")
      (if (`KismetSystemLibrary.DoesImplementInterface` _array_element "/Game/Blueprints/Dialogue/BPI_Talk.BPI_Talk_C")
        (message `/Game/Blueprints/Dialogue/BPI_Talk.Talk` _array_element)))))

(event `Key|E`
  (params (Key :type "Key Structure"))
  ;[1 1 1] Boy Talk
  (:`Pressed`
    (for _array_element (`self.GetOverlappingActors` "/Game/Blueprints/Dialogue/BP_Boy.BP_Boy_C")
      (if (`KismetSystemLibrary.DoesImplementInterface` _array_element "/Game/Blueprints/Dialogue/BPI_Talk.BPI_Talk_C")
        (message `/Game/Blueprints/Dialogue/BPI_Talk.Talk` _array_element)))))

(event `Key|E`
  (params (Key :type "Key Structure"))
  ;[1 1 1] OldWoman Talk
  (:`Pressed`
    (for _array_element (`self.GetOverlappingActors` "/Game/Blueprints/Dialogue/BP_OldWoman.BP_OldWoman_C")
      (if (`KismetSystemLibrary.DoesImplementInterface` _array_element "/Game/Blueprints/Dialogue/BPI_Talk.BPI_Talk_C")
        (message `/Game/Blueprints/Dialogue/BPI_Talk.Talk` _array_element)))))

(event `Key|E`
  (params (Key :type "Key Structure"))
  ;[1 1 1] TempleMan Talk
  (:`Pressed`
    (for _array_element (`self.GetOverlappingActors` "/Game/Blueprints/Dialogue/BP_TempleMan.BP_TempleMan_C")
      (if (`KismetSystemLibrary.DoesImplementInterface` _array_element "/Game/Blueprints/Dialogue/BPI_Talk.BPI_Talk_C")
        (message `/Game/Blueprints/Dialogue/BPI_Talk.Talk` _array_element)))))

(event `Key|E`
  (params (Key :type "Key Structure"))
  ;[1 1 1] Kaira Talk
  (:`Pressed`
    (for _array_element (`self.GetOverlappingActors` "/Game/Blueprints/Dialogue/BP_Kaira.BP_Kaira_C")
      (if (`KismetSystemLibrary.DoesImplementInterface` _array_element "/Game/Blueprints/Dialogue/BPI_Talk.BPI_Talk_C")
        (message `/Game/Blueprints/Dialogue/BPI_Talk.Talk` _array_element)))))

(fn `Uncrouch Obstacle Detection`
  (returns (`Hit?` :type Boolean))
  (bind _returnvalue (`self.K2_GetActorLocation`))
  (bind (_outhit _returnvalue_2) (`KismetSystemLibrary.SphereTraceSingle` :`Start` _returnvalue :`End` (+ _returnvalue (* (`KismetMathLibrary.GetUpVector` (`self.K2_GetActorRotation`)) 115.0)) :`Radius` 15.0 :`TraceChannel` "TraceTypeQuery1" :`DrawDebugType` "ForDuration"))
  (return _returnvalue_2))

(fn `UserConstructionScript`)