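; Level transition trigger that moves the player to another level when BP_Maincharacter overlaps it.
; It matches the current level name (cave, altar, sun god, cabin) to set return flags on GI_MyGameInstance, using DestinationTag to tell a cleared cave exit from a return.
; All branches then share a delayed sequence of sound and WB_Transition fade before opening the target Level with DestinationTag as the options string.
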(event `self.ReceiveActorBeginOverlap`
  (params (OtherActor :type "Actor Object Reference"))
  (cast `/Game/Blueprints/BP_Maincharacter` OtherActor)
  (bind _returnvalue (`GameplayStatics.GetCurrentLevelName` true))
  (if (`KismetStringLibrary.Contains` _returnvalue "Cave_map")
    (bind _asgi_my_game_instance (cast `/Game/Blueprints/GameMode/GI_MyGameInstance` (`GameplayStatics.GetGameInstance`)))
    (if (`KismetStringLibrary.Contains` (`self.DestinationTag`) "CaveExit")
      (set `/Game/Blueprints/GameMode/GI_MyGameInstance.bReturningFromCave` false _asgi_my_game_instance)
      (set `/Game/Blueprints/GameMode/GI_MyGameInstance.bClearFromCave` true _asgi_my_game_instance)
      (else
        (set `/Game/Blueprints/GameMode/GI_MyGameInstance.bReturningFromCave` true _asgi_my_game_instance)
        (set `/Game/Blueprints/GameMode/GI_MyGameInstance.bClearFromCave` false _asgi_my_game_instance)))
    (elif (`KismetStringLibrary.Contains` _returnvalue "Altar")
      (bind _asgi_my_game_instance_2 (cast `/Game/Blueprints/GameMode/GI_MyGameInstance` (`GameplayStatics.GetGameInstance`)))
      (set `/Game/Blueprints/GameMode/GI_MyGameInstance.bReturningFromAlter` true _asgi_my_game_instance_2)
      (elif (`KismetStringLibrary.Contains` _returnvalue "SunGod_Map")
        (bind _asgi_my_game_instance_3 (cast `/Game/Blueprints/GameMode/GI_MyGameInstance` (`GameplayStatics.GetGameInstance`)))
        (set `/Game/Blueprints/GameMode/GI_MyGameInstance.bReturningFromSunGod` true _asgi_my_game_instance_3)
        (elif (`KismetStringLibrary.Contains` "" "Cabin_Map")
          (bind _asgi_my_game_instance_4 (cast `/Game/Blueprints/GameMode/GI_MyGameInstance` (`GameplayStatics.GetGameInstance`)))
          (set `/Game/Blueprints/GameMode/GI_MyGameInstance.bReturningFromCabin` true _asgi_my_game_instance_4)))))
  (`KismetSystemLibrary.Delay` 0.5)
  (`GameplayStatics.PlaySound2D` (`self.Sound`) 1.0 1.0 0.0 null null)
  (`KismetSystemLibrary.Delay` 0.2)
  ;[0.2564 0.8293 1] 트렌지션 시 Fade out
  (bind _returnvalue_2 (`|CreateWidget` "/Game/Blueprints/transition/WB_Transition.WB_Transition_C"))
  (`UserWidget.AddToViewport` _returnvalue_2 0)
  (`/Game/Blueprints/transition/WB_Transition.Play Fade` _returnvalue_2)
  (`KismetSystemLibrary.Delay` 1.0)
  (`GameplayStatics.OpenLevelBySoftObjectPtr` (`self.Level`) true (`self.DestinationTag`)))

(fn `UserConstructionScript`)