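; BP_Robber is the player character for a heist game, with Enhanced Input movement, crouch, montage dodge roll and pause menu.
; BeginPlay creates the health HUD, plus detection meter and timer outside MainMenu.
; Crouching lowers speed, with timelines shrinking the capsule and lengthening the camera arm; an upward sphere trace blocks standing under obstacles.
; External events handle ragdoll, resuming, showing the carried jewel and teleporting to PlayerStart.
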(event `self.ReceiveBeginPlay`
  ;[1 1 1] Input and Movement
  ;[1 1 1] Health System
  (`|ExecutionSequence`
    (:`then_0`
      (bind _returnvalue (`|CreateWidget` "/Game/UI/WB_HealthSystem.WB_HealthSystem_C"))
      (`UserWidget.AddToViewport` _returnvalue 0))
    (:`then_1`
      (`EnhancedInputSubsystemInterface.AddMappingContext` (pcsubsystem `EnhancedInputLocalPlayerSubsystem` (`GameplayStatics.GetPlayerController` 0)) "/Game/Input/IMC_PlayerInput.IMC_PlayerInput" 0 (struct))
      (bind _returnvalue_2 (`GameplayStatics.GetCurrentLevelName` true))
      (if (`KismetStringLibrary.NotEqual_StrStr` _returnvalue_2 "MainMenu")
        (bind _returnvalue_3 (`|CreateWidget` "/Game/UI/WB_DetectionMeter.WB_DetectionMeter_C"))
        (bind _output_get (set `self.Detected Meter Widget` _returnvalue_3))
        (`UserWidget.AddToViewport` _output_get 0)
        (bind _returnvalue_4 (`|CreateWidget` "/Game/UI/WB_Timer.WB_Timer_C"))
        (bind _output_get_2 (set `self.Timer Widget` _returnvalue_4))
        (`UserWidget.AddToViewport` _output_get_2 0)))))

(event `EnhancedInput|/Game/Input/IA_Move`
  (params (ActionValue :type "Vector2D Structure") (ElapsedSeconds :type "Float (double-precision)") (TriggeredSeconds :type "Float (double-precision)") (InputAction :type "InputAction Object Reference" :default "/Game/Input/IA_Move.IA_Move"))
  ;[1 1 1] Input and Movement
  (:`Triggered`
    (`self.AddMovementInput` (`KismetMathLibrary.GetRightVector` (`self.GetControlRotation`)) ActionValue_X)
    (`self.AddMovementInput` (`KismetMathLibrary.GetForwardVector` (`self.GetControlRotation`)) ActionValue_Y)))

(event `EnhancedInput|/Game/Input/IA_Look`
  (params (ActionValue :type "Vector2D Structure") (ElapsedSeconds :type "Float (double-precision)") (TriggeredSeconds :type "Float (double-precision)") (InputAction :type "InputAction Object Reference" :default "/Game/Input/IA_Look.IA_Look"))
  ;[1 1 1] Input and Movement
  (:`Triggered`
    (`self.AddControllerYawInput` ActionValue_X)
    (`self.AddControllerPitchInput` (* ActionValue_Y -1.0))))

(event `EnhancedInput|/Game/Input/IA_Crawl`
  (params (ActionValue :type Boolean) (ElapsedSeconds :type "Float (double-precision)") (TriggeredSeconds :type "Float (double-precision)") (InputAction :type "InputAction Object Reference" :default "/Game/Input/IA_Crawl.IA_Crawl"))
  (bind _charactermovement (`self.CharacterMovement`))
  ;[1 1 1] Crouch
  (:`Started`
    (if (not (`self.crouched`))
      (set `self.crouched` true)
      (set `CharacterMovementComponent.MaxWalkSpeed` 350.0 _charactermovement)
      (`|ExecutionSequence`
        (:`then_0`
          (bind (_direction _arm_length) (`Timeline|Crouch Zoom Out` :!label _label)
            (:`Update`
              (set `SpringArmComponent.TargetArmLength` (`KismetMathLibrary.Lerp` 600.0 750.0 _arm_length) (`self.SpringArm`)))))
        (:`then_1`
          (bind (_direction_2 _capsule_height) (`Timeline|Capsule Height` :!label _label_2)
            (:`Update`
              (`CapsuleComponent.SetCapsuleHalfHeight` (`self.CapsuleComponent`) (`KismetMathLibrary.Lerp` 88.0 50.0 _capsule_height) true)
              (`SceneComponent.K2_SetRelativeLocation` (`self.Mesh`) (`KismetMathLibrary.MakeVector` 0.0 0.0 (`KismetMathLibrary.Lerp` -89.0 -59.0 _capsule_height)) false false)))))
      (else
        (bind _hit_ (`self.Uncrouch Obstacle Detection`))
        (if (not _hit_)
          (set `self.crouched` false)
          (set `CharacterMovementComponent.MaxWalkSpeed` 600.0 _charactermovement)
          (`|ExecutionSequence`
            (:`then_0`
              (goto _label :!via `Reverse`))
            (:`then_1`
              (goto _label_2 :!via `Reverse`))))))))

(event `EnhancedInput|/Game/Input/IA_Roll`
  (params (ActionValue :type Boolean) (ElapsedSeconds :type "Float (double-precision)") (TriggeredSeconds :type "Float (double-precision)") (InputAction :type "InputAction Object Reference" :default "/Game/Input/IA_Roll.IA_Roll"))
  ;[1 1 1] Dodge Roll
  (:`Started`
    (if (not (`self.is dodging?`))
      (`|PlayMontage` (`self.Mesh`) "/Game/Characters/Robber/Roll/Roll_Montage.Roll_Montage"
        (:`then`
          (set `self.is dodging?` true))
        (:`OnCompleted`
          (set `self.is dodging?` false))))))

(event `Ragdoll`
  (`PrimitiveComponent.SetSimulatePhysics` (`self.Mesh`) true)
  (`self.DisableInput` null))

(event `EnhancedInput|/Game/Input/IA_Pause`
  (params (ActionValue :type Boolean) (ElapsedSeconds :type "Float (double-precision)") (TriggeredSeconds :type "Float (double-precision)") (InputAction :type "InputAction Object Reference" :default "/Game/Input/IA_Pause.IA_Pause"))
  (bind _returnvalue (`GameplayStatics.GetPlayerController` 0))
  (bind _returnvalue_2 (`GameplayStatics.GetPlayerController` 0))
  (:`Started`
    (if (not (`self.paused?`))
      (set `self.paused?` true)
      (bind _returnvalue_3 (`|CreateWidget` "/Game/UI/WB_PauseMenu.WB_PauseMenu_C"))
      (bind _output_get (set `self.Pause Menu Widget` _returnvalue_3))
      (`UserWidget.AddToViewport` _output_get 0)
      (set `PlayerController.bShowMouseCursor` true _returnvalue_2)
      (`WidgetBlueprintLibrary.SetInputMode_GameAndUIEx` _returnvalue_2 (`self.Pause Menu Widget`))
      (`GameplayStatics.SetGamePaused` true)
      (else
        (bind _pause_menu_widget (`self.Pause Menu Widget` :!label _label_3)
          (:`then`
            (`Widget.RemoveFromParent` _pause_menu_widget)
            (set `self.Pause Menu Widget` null)
            (set `self.paused?` false)
            (set `PlayerController.bShowMouseCursor` false _returnvalue)
            (`WidgetBlueprintLibrary.SetInputMode_GameOnly` _returnvalue)
            (`GameplayStatics.SetGamePaused` false))
          (:`else`))))))

(event `Resume`
  (goto _label_3))

(event `Equip Jewel`
  (`SceneComponent.SetVisibility` (`self.Jewel`) true false)
  (set `self.hasJewel` true))

(event `Go To Start`
  (bind _returnvalue (`GameplayStatics.GetActorOfClass` "/Script/Engine.PlayerStart"))
  (`self.K2_SetActorLocation` (`self.K2_GetActorLocation` _returnvalue)))

(fn `Uncrouch Obstacle Detection`
  (returns (`Hit?` :type Boolean))
  (bind _returnvalue (`self.K2_GetActorLocation`))
  (bind (_outhit _returnvalue_2) (`KismetSystemLibrary.SphereTraceSingle` :`Start` _returnvalue :`End` (+ _returnvalue (* (`KismetMathLibrary.GetUpVector` (`self.K2_GetActorRotation`)) 115.0)) :`Radius` 15.0 :`TraceChannel` "TraceTypeQuery1" :`DrawDebugType` "ForDuration"))
  (return _returnvalue_2))

(fn `UserConstructionScript`)