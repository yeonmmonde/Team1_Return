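; Stealth game mode that runs the level's music and rain audio and handles the player getting captured.
; BeginPlay starts the music and rain loop, and SwitchMusictoEscaping swaps the music for the escape track.
; Captured shows a fading captured widget with UI input enabled.
; If escape music exists, it also fades that out, plays the caught sound, silences BP_Alarm and ragdolls the BP_Robber player.
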(event `self.ReceiveBeginPlay`
  (bind _returnvalue (`GameplayStatics.GetPlayerController` 0))
  (bind _returnvalue_2 (`GameplayStatics.SpawnSound2D` "/Game/Audio/Music/Music.Music" 0.3 1.0 0.0 null))
  (bind _output_get (set `self.Music` _returnvalue_2))
  (`AudioComponent.FadeIn` _output_get 0.3 1.0 0.0 "Linear")
  (bind _returnvalue_3 (`GameplayStatics.SpawnSound2D` "/Game/Audio/Effect/Rain_Loop.Rain_Loop" 0.3 1.0 0.0 null))
  (bind _output_get_2 (set `self.Rain Loop` _returnvalue_3))
  (`AudioComponent.FadeIn` _output_get_2 0.0 1.0 0.0 "Linear")
  (set `PlayerController.bShowMouseCursor` true _returnvalue)
  (`WidgetBlueprintLibrary.SetInputMode_GameOnly` _returnvalue))

(event `Captured`
  (bind _returnvalue (`GameplayStatics.GetPlayerController` 0))
  (set `PlayerController.bShowMouseCursor` true _returnvalue)
  (`WidgetBlueprintLibrary.SetInputMode_GameAndUIEx` _returnvalue null)
  (bind _returnvalue_2 (`|CreateWidget` "/Game/UI/WB_Captured.WB_Captured_C"))
  (bind _output_get (set `self.Captured Widget` _returnvalue_2))
  (`UserWidget.AddToViewport` _output_get 0)
  (`/Game/UI/WB_Captured.Play Fade Animation` (`self.Captured Widget`))
  (bind _escaping_music (`self.Escaping Music`)
    (:`then`
      (`AudioComponent.FadeOut` _escaping_music 0.3 0.0 "Linear")
      (`GameplayStatics.PlaySound2D` "/Game/Audio/Effect/Caught.Caught" 1.0 1.0 0.0 null null)
      (bind _returnvalue_3 (`GameplayStatics.GetActorOfClass` "/Game/Blueprints/Sensors_Alarms/BP_Alarm.BP_Alarm_C"))
      (`AudioComponent.FadeOut` (`/Game/Blueprints/Sensors_Alarms/BP_Alarm.Alarm Sound` _returnvalue_3) 0.0 0.0 "Linear")
      (bind _asbp_robber (cast `/Game/Blueprints/BP_Robber` (`GameplayStatics.GetPlayerCharacter` 0)))
      (`/Game/Blueprints/BP_Robber.Ragdoll` _asbp_robber))
    (:`else`)))

(event `Switch Music to Escaping`
  (`AudioComponent.FadeOut` (`self.Music`) 0.3 0.0 "Linear")
  (bind _returnvalue (`GameplayStatics.SpawnSound2D` "/Game/Audio/Music/Escaping.Escaping" 0.5 1.0 0.0 null))
  (set `self.Escaping Music` _returnvalue))

(fn `UserConstructionScript`)