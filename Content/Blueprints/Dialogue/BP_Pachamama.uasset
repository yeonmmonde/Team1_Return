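; Pachamama dialogue actor that drives level music, a reveal sequence and a memory video.
; BeginPlay starts the first BGM and picks Dialogue1 by the game instance's HasHeart and IsKorean flags, hiding meshes and trigger in the Korean with-heart branch.
; The colision event, commented as firing on talk, repositions those components, crossfades music and spawns a level-up particle.
; Player overlap with the Video component fades out music and shows the memory video widget.
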(event `self.video.OnComponentBeginOverlap`
  (params (OverlappedComponent :type "PrimitiveComponent Object Reference") (OtherActor :type "Actor Object Reference") (OtherComp :type "PrimitiveComponent Object Reference") (OtherBodyIndex :type Integer) (bFromSweep :type Boolean) (SweepResult :type "HitResult Structure (by ref)"))
  ;[1 1 1] video
  (cast `/Game/Blueprints/BP_Maincharacter` OtherActor)
  (`|ExecutionSequence`
    (:`then_0`
      (if (`KismetSystemLibrary.IsValid` (`self.Bgm 2`))
        (`AudioComponent.FadeOut` (`self.Bgm 2`) 3.0 0.2 "Linear")
        (bind _returnvalue (`|CreateWidget` "/Game/Blueprints/pachamamaplay/WB_MemoryVideo_A05.WB_MemoryVideo_A05_C" :!label _label))
        (`/Game/Blueprints/pachamamaplay/WB_MemoryVideo_A05.Remove video` _returnvalue)
        (`UserWidget.AddToViewport` _returnvalue 0)))
    (:`then_1`
      (if (`KismetSystemLibrary.IsValid` (`self.Bgm1`))
        (`AudioComponent.FadeOut` (`self.Bgm1`) 3.0 0.2 "Linear")
        (goto _label)))))

(event `colision`
  (`KismetSystemLibrary.Delay` 0.4)
  (`|ExecutionSequence`
    (:`then_0`
      (`SceneComponent.K2_SetRelativeLocation` (`self.StaticMesh1`) (0.0 33.896193 169.097619) false false))
    (:`then_1`
      (`SceneComponent.K2_SetRelativeLocationAndRotation` (`self.StaticMesh`) (0.0 0.0 -79.350968) (struct :`Yaw` -89.9) false false))
    (:`then_2`
      (`SceneComponent.K2_SetRelativeLocation` (`self.Trigger Zone`) (375.870543 0.0 -91.56555) false false))
    (:`then_3`
      (`SceneComponent.SetVisibility` (`self.StaticMesh1`) true false))
    (:`then_4`
      ;[0.7881 0.4766 1] 말걸었을때 음악 바뀌게
      (`AudioComponent.FadeOut` (`self.Bgm1`) 3.0 0.0 "Linear")
      (bind _returnvalue (`GameplayStatics.SpawnSound2D` "/Game/Audio/Music/Low_Noon_-_John_Patitucci.Low_Noon_-_John_Patitucci" 1.0 1.0 0.0 null false false))
      (bind _output_get (set `self.Bgm 2` _returnvalue))
      (`AudioComponent.FadeIn` _output_get 3.0 1.0 0.0 "Linear")
      (`KismetSystemLibrary.Delay` 1.0)
      (`GameplayStatics.SpawnEmitterAtLocation` "/Game/Effect/InfinityBladeEffects/Effects/FX_Mobile/Misc/P_levelUp_Detail3.P_levelUp_Detail3" (-1180.667589 -2240.525869 2236.758868) (struct) (0.5 0.5 0.5)))))

(event `self.ReceiveBeginPlay`
  (`|ExecutionSequence`
    (:`then_0`
      ;[1 1 1] bgm
      (bind _returnvalue (`GameplayStatics.SpawnSound2D` "/Game/Audio/Music/In_the_Temple_Garden.In_the_Temple_Garden" 1.0 1.0 0.0 null false false))
      (set `self.Bgm1` _returnvalue))
    (:`then_1`
      (bind _asgi_my_game_instance (cast `/Game/Blueprints/GameMode/GI_MyGameInstance` (`GameplayStatics.GetGameInstance`)))
      (if (`/Game/Blueprints/GameMode/GI_MyGameInstance.HasHeart` _asgi_my_game_instance)
        (if (`/Game/Blueprints/GameMode/GI_MyGameInstance.bIsKorean` _asgi_my_game_instance)
          (set `self.dialogue1` (`self.K_dialogue1`))
          (`SceneComponent.K2_SetRelativeLocationAndRotation` :`self` (`self.StaticMesh`) :`NewLocation` (0.0 0.0 -1000.0))
          (`SceneComponent.K2_SetRelativeLocationAndRotation` :`self` (`self.Trigger Zone`) :`NewLocation` (0.0 0.0 -1000.0))
          (`SceneComponent.K2_SetRelativeLocationAndRotation` :`self` (`self.StaticMesh1`) :`NewLocation` (0.0 0.0 -1000.0))
          (`SceneComponent.SetVisibility` (`self.StaticMesh1`) false false))
        (else
          (set `self.dialogue1` (`self.NoHeartDialogue`))
          (if (`/Game/Blueprints/GameMode/GI_MyGameInstance.bIsKorean` _asgi_my_game_instance)
            (set `self.dialogue1` (`self.K_NoHeartDialogue`))))))))

(fn `UserConstructionScript`
  (`parent.UserConstructionScript`))