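; BP_PachamamaPlay is an altar interaction that reveals a hidden orb and triggers a memory video.
; Overlapping Sphere1 shows a prompt, freezes the main character and enables E input.
; E runs a delayed sequence: particle burst at a fixed location, orb reveal, movement restored, pause-menu Sequence2 shown, trigger removed.
; Character overlap with Colision destroys the actor and adds the WB_MemoryVideo_A01 widget to the viewport.
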(event `self.ReceiveBeginPlay`
  (`SceneComponent.SetVisibility` (`self.Sphere`) false false)
  (`SceneComponent.SetVisibility` (`self.colision`) false false))

(event `view orb`
  ;[1 1 1] 아이템
  (`SceneComponent.SetVisibility` (`self.Sphere`) true false)
  (`SceneComponent.SetVisibility` (`self.colision`) true false))

(event `Key|E`
  (params (Key :type "Key Structure"))
  (:`Pressed`
    (bind _output_get (set `self.IsPressE?` true))
    (if _output_get :!label _label
      (`SceneComponent.SetVisibility` (`self.Widget`) false false)
      (`KismetSystemLibrary.Delay` 0.2)
      (bind _returnvalue (`GameplayStatics.SpawnEmitterAtLocation` "/Game/Effect/InfinityBladeEffects/Effects/FX_Mobile/Misc/P_levelUp_Detail2.P_levelUp_Detail2" (65.0 -650.0 275.0) (struct) (0.5 0.5 0.5)))
      (`KismetSystemLibrary.Delay` 1.0)
      (`self.view orb`)
      (`KismetSystemLibrary.Delay` 5.0)
      (`ActorComponent.K2_DestroyComponent` _returnvalue)
      (`/Game/Blueprints/BP_Maincharacter.enable movement` (stale `self.Sphere1.OnComponentBeginOverlap` _asbp_maincharacter))
      (`Widget.SetVisibility` (`/Game/Blueprints/UI/WB_PauseMenu.Sequence2` (`/Game/Blueprints/BP_Maincharacter.Pause Menu Widget` (stale `self.Sphere1.OnComponentBeginOverlap` _asbp_maincharacter))) "Visible")
      (`ActorComponent.K2_DestroyComponent` (`self.Sphere1`)))))

(event `self.Sphere1.OnComponentBeginOverlap`
  (params (OverlappedComponent :type "PrimitiveComponent Object Reference") (OtherActor :type "Actor Object Reference") (OtherComp :type "PrimitiveComponent Object Reference") (OtherBodyIndex :type Integer) (bFromSweep :type Boolean) (SweepResult :type "HitResult Structure (by ref)"))
  ;[1 1 1] 위젯
  (`SceneComponent.SetVisibility` (`self.Widget`) true false)
  (bind _asbp_maincharacter (cast `/Game/Blueprints/BP_Maincharacter` OtherActor))
  (`/Game/Blueprints/BP_Maincharacter.disable movement` _asbp_maincharacter)
  (`self.EnableInput` (`GameplayStatics.GetPlayerController` 0))
  (goto _label))

(event `self.Sphere1.OnComponentEndOverlap`
  (params (OverlappedComponent :type "PrimitiveComponent Object Reference") (OtherActor :type "Actor Object Reference") (OtherComp :type "PrimitiveComponent Object Reference") (OtherBodyIndex :type Integer))
  ;[1 1 1] 위젯
)

(event `self.colision.OnComponentBeginOverlap`
  (params (OverlappedComponent :type "PrimitiveComponent Object Reference") (OtherActor :type "Actor Object Reference") (OtherComp :type "PrimitiveComponent Object Reference") (OtherBodyIndex :type Integer) (bFromSweep :type Boolean) (SweepResult :type "HitResult Structure (by ref)"))
  ;[1 1 1] 영상플레이
  (bind _asbp_maincharacter (cast `/Game/Blueprints/BP_Maincharacter` OtherActor))
  (set `self.As BP Maincharacter` _asbp_maincharacter)
  (`self.K2_DestroyActor`)
  (bind _returnvalue (`|CreateWidget` "/Game/map/Altar/blueprint/WB_MemoryVideo_A01.WB_MemoryVideo_A01_C"))
  (`/Game/map/Altar/blueprint/WB_MemoryVideo_A01.Remove video` _returnvalue)
  (`UserWidget.AddToViewport` _returnvalue 0))

(fn `UserConstructionScript`)