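; BP_Respawn is a child Blueprint in the MainTree map folder that, by its name, serves as a respawn actor.
; On overlap, it casts the other actor to BP_Maincharacter and reads HasHeart from that character's GameInstance.
; It forwards the overlap to the parent class only when HasHeart is true, so it acts as a condition gate on inherited behavior.
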(event `self.ReceiveActorBeginOverlap`
  (params (OtherActor :type "Actor Object Reference"))
  (bind _asbp_maincharacter (cast `/Game/Blueprints/BP_Maincharacter` OtherActor))
  (if (`/Game/Blueprints/GameMode/GI_MyGameInstance.HasHeart` (`/Game/Blueprints/BP_Maincharacter._GameInstance` _asbp_maincharacter))
    (`parent.ReceiveActorBeginOverlap` OtherActor)))

(fn `UserConstructionScript`
  (`parent.UserConstructionScript`))