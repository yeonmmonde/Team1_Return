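; Prayer-point actor for the Pachamama play area that awards the first memory orb and launches its memory video.
; Overlapping Sphere1 shows a prompt, locks player movement and enables E input.
; Pressing E runs a delay-paced sequence: pray, particle burst, orb reveal, timeline-driven light and transition widget.
; It then unlocks a pause-menu play button, flags the GameInstance, opens the video widget, fires pray dispatchers, destroys itself and restores movement.
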(event `self.ReceiveBeginPlay`
  (`SceneComponent.SetVisibility` (`self.Sphere`) false false)
  (`SceneComponent.SetVisibility` (`self.colision`) false false))

(event `PlaySequence2`
  ;[1 1 1] 영상플레이
  (`|ExecutionSequence`
    (:`then_0`
      (bind _returnvalue (`|CreateWidget` "/Game/Blueprints/pachamamaplay/WB_MemoryVideo_A02.WB_MemoryVideo_A02_C"))
      (`/Game/Blueprints/pachamamaplay/WB_MemoryVideo_A02.Remove video` _returnvalue)
      (`UserWidget.AddToViewport` _returnvalue 0)
      (`self.DonePray`)
      (`self.K2_DestroyActor`))
    (:`then_1`
      (`self.OnPray`))))

(event `view orb`
  ;[1 1 1] 아이템
  (`SceneComponent.SetVisibility` (`self.Sphere`) true false)
  (`SceneComponent.SetVisibility` (`self.colision`) true false))

(event `Key|E`
  (params (Key :type "Key Structure"))
  ;[1 1 1] 코멘트
  (:`Pressed`
    (bind _output_get (set `self.IsPressE?` true))
    (if _output_get :!label _label
      (`SceneComponent.SetVisibility` (`self.Widget`) false false)
      (`/Game/Blueprints/BP_Maincharacter.pray` (stale `self.Sphere1.OnComponentBeginOverlap` _asbp_maincharacter))
      (`KismetSystemLibrary.Delay` 1.5)
      (bind _returnvalue (`GameplayStatics.SpawnEmitterAtLocation` "/Game/Effect/InfinityBladeEffects/Effects/FX_Mobile/Misc/P_levelUp_Detail2.P_levelUp_Detail2" (15.0 -600.0 300.0) (struct) (0.5 0.5 0.5)))
      (`KismetSystemLibrary.Delay` 1.0)
      (`self.view orb`)
      ;[1 1 1] 빛
      (bind (_direction _light) (`Timeline|lighter`)
        (:`Update`
          (`LightComponent.SetIntensity` (`self.PointLight`) _light)
          (`KismetSystemLibrary.Delay` 3.4)
          ;[0.2564 0.8293 1] 트렌지션후  Fade in
          (bind _returnvalue_2 (`|CreateWidget` "/Game/Blueprints/transition/WB_SequenceTransition.WB_SequenceTransition_C"))
          (`UserWidget.AddToViewport` _returnvalue_2 0)
          (`KismetSystemLibrary.Delay` 2.0)
          (`Widget.SetVisibility` (`/Game/Blueprints/UI/WB_PauseMenu.PlayButton_2` (`/Game/Blueprints/BP_Maincharacter.Pause Menu Widget` (stale `self.Sphere1.OnComponentBeginOverlap` _asbp_maincharacter))) "Visible")
          (bind _asgi_my_game_instance (cast `/Game/Blueprints/GameMode/GI_MyGameInstance` (`GameplayStatics.GetGameInstance`)))
          (set `/Game/Blueprints/GameMode/GI_MyGameInstance.bIsGetMemoryBall_First` true _asgi_my_game_instance)
          (`ActorComponent.K2_DestroyComponent` (`self.Sphere1`))
          (`ActorComponent.K2_DestroyComponent` _returnvalue)
          (`self.PlaySequence2`)
          (`Widget.SetVisibility` _returnvalue_2 "Hidden")
          (`/Game/Blueprints/BP_Maincharacter.enable movement` (stale `self.Sphere1.OnComponentBeginOverlap` _asbp_maincharacter)))))))

(event `self.Sphere1.OnComponentBeginOverlap`
  (params (OverlappedComponent :type "PrimitiveComponent Object Reference") (OtherActor :type "Actor Object Reference") (OtherComp :type "PrimitiveComponent Object Reference") (OtherBodyIndex :type Integer) (bFromSweep :type Boolean) (SweepResult :type "HitResult Structure (by ref)"))
  ;[1 1 1] 위젯
  (`SceneComponent.SetVisibility` (`self.Widget`) true false)
  (bind _asbp_maincharacter (cast `/Game/Blueprints/BP_Maincharacter` OtherActor))
  (`/Game/Blueprints/BP_Maincharacter.disable movement` _asbp_maincharacter)
  (`self.EnableInput` (`GameplayStatics.GetPlayerController` 0))
  (goto _label))

(event `self.Sphere1.OnComponentEndOverlap`
  (params (OverlappedComponent :type "PrimitiveComponent Object Reference") (OtherActor :type "Actor Object Reference") (OtherComp :type "PrimitiveComponent Object Reference") (OtherBodyIndex :type Integer))
  ;[1 1 1] 위젯
)

(fn `UserConstructionScript`)