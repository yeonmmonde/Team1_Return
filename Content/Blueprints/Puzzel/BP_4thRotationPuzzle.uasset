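; Four-ring rotation puzzle actor that the player attaches to at the nearest Handle socket, with the view switched to a puzzle camera.
; Tab cycles the highlighted ring, and move input turns it and the handle one 36-degree step through a self-recalling delayed event, also rotating linked rings from RollWith arrays.
; Each step updates the rings' digits, and when the combined four-digit number matches TotalScore it fires EventActor, spawns DropItem and releases the player.
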(event `self.ReceiveBeginPlay`
  (set `self.ActiveCircle` (`self.Ring_X`)))

(event `self.ReceiveTick`
  (params (DeltaSeconds :type "Float (single-precision)"))
  ;[1 1 1] 위젯 띄우기
  (bind _asbp_maincharacter (cast `/Game/Blueprints/BP_Maincharacter` (`GameplayStatics.GetPlayerCharacter` 0)))
  (`SceneComponent.K2_SetWorldRotation` (`self.InteractionWidget`) (`KismetMathLibrary.Conv_VectorToRotator` (* (`SceneComponent.GetForwardVector` (`/Game/Blueprints/BP_Maincharacter.Camera` _asbp_maincharacter)) -1.0)) false false))

(event `self.Box.OnComponentBeginOverlap`
  (params (OverlappedComponent :type "PrimitiveComponent Object Reference") (OtherActor :type "Actor Object Reference") (OtherComp :type "PrimitiveComponent Object Reference") (OtherBodyIndex :type Integer) (bFromSweep :type Boolean) (SweepResult :type "HitResult Structure (by ref)"))
  (bind _interactionwidget (`self.InteractionWidget`))
  ;[1 1 1] 위젯 띄우기
  (bind _asbp_maincharacter (cast `/Game/Blueprints/BP_Maincharacter` OtherActor))
  (`SceneComponent.K2_SetWorldRotation` _interactionwidget (`KismetMathLibrary.Conv_VectorToRotator` (* (`SceneComponent.GetForwardVector` (`/Game/Blueprints/BP_Maincharacter.Camera` _asbp_maincharacter)) -1.0)) false false)
  (`SceneComponent.SetVisibility` _interactionwidget true false)
  (set `self.IsReady` true)
  (set `/Game/Blueprints/BP_Maincharacter.Interact4thPuzzle` self _asbp_maincharacter))

(event `self.Box.OnComponentEndOverlap`
  (params (OverlappedComponent :type "PrimitiveComponent Object Reference") (OtherActor :type "Actor Object Reference") (OtherComp :type "PrimitiveComponent Object Reference") (OtherBodyIndex :type Integer))
  ;[1 1 1] 위젯 지우기
  (bind _asbp_maincharacter (cast `/Game/Blueprints/BP_Maincharacter` OtherActor))
  (set `/Game/Blueprints/BP_Maincharacter.Interact4thPuzzle` null _asbp_maincharacter)
  (`SceneComponent.SetVisibility` (`self.InteractionWidget`) false false)
  (set `self.IsReady` false))

(event `self.Talk`
  (bind _returnvalue (`GameplayStatics.GetPlayerCharacter` 0))
  (bind _returnvalue_2 (`GameplayStatics.GetPlayerController` 0))
  (bind _returnvalue_3 (`GameplayStatics.GetPlayerCharacter` 0))
  (bind _handle (`self.Handle`))
  (bind _ring_l (`self.Ring_L`))
  (bind (_returnvalue_location _returnvalue_rotation) (`KismetMathLibrary.BreakTransform` (`SceneComponent.GetSocketTransform` (`self.Handle`) (`self.ShortestLocationName`) "RTS_World")))
  ;[1 1 1] 붙이기
  (if (`self.IsAttachPlayer`)
    (`CharacterMovementComponent.SetMovementMode` (`Character.CharacterMovement` _returnvalue) "MOVE_Walking" 0)
    (set `self.IsAttachPlayer` false)
    (`self.EnableInput` _returnvalue_2)
    (`self.SetOwner` _returnvalue null)
    (`self.SetNormalMaterial` (`self.ActiveCircle`))
    (set `self.ActiveCircle` _ring_l)
    (`SceneComponent.K2_SetRelativeRotation` _ring_l (struct :`Yaw` 180.0) false false)
    (`SceneComponent.K2_SetRelativeRotation` (`self.Ring_M`) (struct :`Yaw` 180.0) false false)
    (`SceneComponent.K2_SetRelativeRotation` (`self.Ring_S`) (struct :`Yaw` 180.0) false false)
    (`SceneComponent.K2_SetRelativeRotation` (`self.Ring_X`) (struct :`Yaw` 180.0) false false)
    (`SceneComponent.SetVisibility` (`self.InteractionWidget`) true false)
    (set `self.ShortestLocation` 999.0)
    (set `self.s` 0)
    (set `self.m` 0)
    (set `self.l` 0)
    ;[1 1 1] 돌리기
    (set `self.X` 0)
    (`PlayerController.SetViewTargetWithBlend` (`GameplayStatics.GetPlayerController` 0) (`GameplayStatics.GetPlayerCharacter` 0) 0.0 "VTBlend_Linear" 0.0 false)
    (bind _asbp_maincharacter (cast `/Game/Blueprints/BP_Maincharacter` (`GameplayStatics.GetPlayerCharacter` 0)))
    (set `/Game/Blueprints/BP_Maincharacter.InteractBigPuzzle` null _asbp_maincharacter)
    (else
      (`SceneComponent.SetVisibility` (`self.InteractionWidget`) false false)
      (`PlayerController.SetViewTargetWithBlend` _returnvalue_2 (`self.Camera`) 0.0 "VTBlend_Linear" 0.0 false)
      (for _array_element (`SceneComponent.GetAllSocketNames` _handle)
        (bind _returnvalue_4 (`KismetMathLibrary.Vector_Distance` (`SceneComponent.GetSocketLocation` _handle _array_element) (`self.K2_GetActorLocation` (`GameplayStatics.GetPlayerCharacter` 0))))
        (if (<= _returnvalue_4 (`self.ShortestLocation`))
          (set `self.ShortestLocation` _returnvalue_4)
          (set `self.ShortestLocationName` _array_element)))
      (bind _returnvalue_5 (`self.K2_AttachToComponent` (`GameplayStatics.GetPlayerCharacter` 0) (`self.Handle`) (`self.ShortestLocationName`) "KeepWorld" "KeepRelative" "KeepRelative" true))
      (set `self.IsAttachPlayer` _returnvalue_5)
      (`CharacterMovementComponent.DisableMovement` (`Character.CharacterMovement` _returnvalue_3))
      (`self.K2_SetActorLocationAndRotation` _returnvalue_3 _returnvalue_location _returnvalue_rotation false false)
      (`self.SetActiveMaterial` (`self.ActiveCircle`)))))

(event `Tab`
  (bind _activecircle (`self.ActiveCircle`))
  ;[1 1 1] 기본 머테리얼로 변경
  (`self.SetNormalMaterial` (`self.ActiveCircle`))
  ;[1 1 1] 활성 원 변경
  (if (== _activecircle (`self.Ring_S`))
    (set `self.ActiveCircle` (`self.Ring_X`))
    (elif (== _activecircle (`self.Ring_M`))
      (set `self.ActiveCircle` (`self.Ring_S`))
      (elif (== _activecircle (`self.Ring_L`))
        (set `self.ActiveCircle` (`self.Ring_M`))
        (else
          (set `self.ActiveCircle` (`self.Ring_L`))))))
  (`self.SetActiveMaterial` (`self.ActiveCircle`)))

(event `self.MoveInteraction`
  (params (MoveDir :type "Float (double-precision)"))
  ;[1 1 1] 돌리기
  (if (!= MoveDir 0.0)
    (set `self.IsRolling` true)
    (if (!= (`self.RollCount`) 36.0)
      (`SceneComponent.K2_AddLocalRotation` (`self.Handle`) (`KismetMathLibrary.MakeRotator` 0.0 0.0 (* MoveDir -1.0)) false false)
      (if (> MoveDir 0.0)
        (`self.RightTurn`)
        (else
          (`self.LeftTurn`)))
      (`KismetSystemLibrary.Delay` 0.01)
      (`/Engine/EditorBlueprintResources/StandardMacros.IncrementFloat` (`self.RollCount`)
        (:`  `
          (`/Game/Blueprints/Puzzel/BPI_Move.MoveInteraction` MoveDir)))
      (else
        (set `self.RollCount` 0.0)
        (set `self.IsRolling` false)
        (`self.CalculateScore`)))))

(event `LeftTurn`
  (bind _activecircle (`self.ActiveCircle`))
  ;[1 1 1] 정방향
  (if (== _activecircle (`self.Ring_S`))
    (`SceneComponent.K2_AddLocalRotation` (`self.Ring_S`) (struct :`Yaw` -1.0) false false)
    (for _array_element (`self.RollWithS`)
      (bind (_combinewith _rollcount) (break `/Game/Blueprints/Puzzel/RotationSystem` _array_element))
      (bind _object (`self.SetRollStruct` _combinewith))
      (`SceneComponent.K2_AddLocalRotation` _object (`KismetMathLibrary.MakeRotator` 0.0 0.0 (`KismetMathLibrary.Conv_IntToDouble` (* _rollcount -1))) false false))
    (if (not (!= (`self.RollCount`) 35.0))
      (`/Engine/EditorBlueprintResources/StandardMacros.IncrementInt` (`self.s`)
        (:`  `
          (`self.CalculateSML` (`self.RollWithS`) 1))))
    (elif (== _activecircle (`self.Ring_M`))
      (`SceneComponent.K2_AddLocalRotation` (`self.Ring_M`) (struct :`Yaw` -1.0) false false)
      (for _array_element_2 (`self.RollWithM`)
        (bind (_combinewith_2 _rollcount_2) (break `/Game/Blueprints/Puzzel/RotationSystem` _array_element_2))
        (bind _object_2 (`self.SetRollStruct` _combinewith_2))
        (`SceneComponent.K2_AddLocalRotation` _object_2 (`KismetMathLibrary.MakeRotator` 0.0 0.0 (`KismetMathLibrary.Conv_IntToDouble` (* _rollcount_2 -1))) false false))
      (if (not (!= (`self.RollCount`) 35.0))
        (`/Engine/EditorBlueprintResources/StandardMacros.IncrementInt` (`self.m`)
          (:`  `
            (`self.CalculateSML` (`self.RollWithM`) 1))))
      (elif (== _activecircle (`self.Ring_L`))
        (`SceneComponent.K2_AddLocalRotation` (`self.Ring_L`) (struct :`Yaw` -1.0) false false)
        (for _array_element_3 (`self.RollWithL`)
          (bind (_combinewith_3 _rollcount_3) (break `/Game/Blueprints/Puzzel/RotationSystem` _array_element_3))
          (bind _object_3 (`self.SetRollStruct` _combinewith_3))
          (`SceneComponent.K2_AddLocalRotation` _object_3 (`KismetMathLibrary.MakeRotator` 0.0 0.0 (`KismetMathLibrary.Conv_IntToDouble` (* _rollcount_3 -1))) false false))
        (if (not (!= (`self.RollCount`) 35.0))
          (`/Engine/EditorBlueprintResources/StandardMacros.IncrementInt` (`self.l`)
            (:`  `
              (`self.CalculateSML` (`self.RollWithL`) 1))))
        (else
          (`SceneComponent.K2_AddLocalRotation` (`self.Ring_X`) (struct :`Yaw` -1.0) false false)
          (for _array_element_4 (`self.RollWithX`)
            (bind (_combinewith_4 _rollcount_4) (break `/Game/Blueprints/Puzzel/RotationSystem` _array_element_4))
            (bind _object_4 (`self.SetRollStruct` _combinewith_4))
            (`SceneComponent.K2_AddLocalRotation` _object_4 (`KismetMathLibrary.MakeRotator` 0.0 0.0 (`KismetMathLibrary.Conv_IntToDouble` (* _rollcount_4 -1))) false false))
          (if (not (!= (`self.RollCount`) 35.0))
            (`/Engine/EditorBlueprintResources/StandardMacros.IncrementInt` (`self.X`)
              (:`  `
                (`self.CalculateSML` (`self.RollWithX`) 1)))))))))

(event `CalculateScore`
  (bind _cameraposition (`self.CameraPosition`))
  (bind _eventactor (`self.EventActor`))
  (bind _dropitem (`self.DropItem`))
  ;[1 1 1] 점수 계산
  (bind _output_get (set `self.s` (mod (`self.s`) 10)))
  (if (not (>= _output_get 0))
    (set `self.s` (+ (`self.s`) 10)))
  (bind _output_get_2 (set `self.m` (mod (`self.m`) 10)))
  (if (not (>= _output_get_2 0))
    (set `self.m` (+ (`self.m`) 10)))
  (bind _output_get_3 (set `self.l` (mod (`self.l`) 10)))
  (if (not (>= _output_get_3 0))
    (set `self.l` (+ (`self.l`) 10)))
  (bind _output_get_4 (set `self.X` (mod (`self.X`) 10)))
  (if (not (>= _output_get_4 0))
    (set `self.X` (+ (`self.X`) 10)))
  (bind _output_get_5 (set `self.NowScore` (+ (`self.s`) (* (`self.m`) 10) (* (`self.l`) 100) (* (`self.X`) 1000))))
  (if (== _output_get_5 (`self.TotalScore`))
    (set `self.IsClear` true)
    (`/Engine/EditorBlueprintResources/StandardMacros.IsValid` _eventactor
      (:`Is Valid`
        (`/Game/Blueprints/PuzzelCustomEvent/BP_ParentCustomEvent.CustomEvent` _eventactor))
      (:`Is Not Valid`
        _))
    (if (`KismetSystemLibrary.IsValidClass` _dropitem)
      (`|SpawnActorFromClass` _dropitem (`SceneComponent.GetSocketTransform` (`self.Sphere`) "None" "RTS_World") "Undefined" "MultiplyWithRoot" null null))
    (`self.K2_SetActorLocationAndRotation` (`self.Camera`) (`SceneComponent.K2_GetComponentLocation` _cameraposition) (`SceneComponent.K2_GetComponentRotation` _cameraposition) false false)
    (`self.DisableInput` (`GameplayStatics.GetPlayerController` 0))
    (`KismetSystemLibrary.Delay` 2.0)
    (`/Game/Blueprints/Dialogue/BPI_Talk.Talk`)))

(event `ClearEvent`
  (bind _dropitem (`self.DropItem`))
  (if (`KismetSystemLibrary.IsValidClass` _dropitem)
    (`|SpawnActorFromClass` _dropitem (`SceneComponent.GetSocketTransform` (`self.Sphere`) "None" "RTS_World") "Undefined" "MultiplyWithRoot" null null)))

(event `RightTurn`
  (bind _activecircle (`self.ActiveCircle`))
  ;[1 1 1] 역방향
  (if (== _activecircle (`self.Ring_S`))
    (`SceneComponent.K2_AddLocalRotation` (`self.Ring_S`) (struct :`Yaw` 1.0) false false)
    (for _array_element (`self.RollWithS`)
      (bind (_combinewith _rollcount) (break `/Game/Blueprints/Puzzel/RotationSystem` _array_element))
      (bind _object (`self.SetRollStruct` _combinewith))
      (`SceneComponent.K2_AddLocalRotation` _object (`KismetMathLibrary.MakeRotator` 0.0 0.0 (`KismetMathLibrary.Conv_IntToDouble` _rollcount)) false false))
    (if (not (!= (`self.RollCount`) 35.0))
      (`/Engine/EditorBlueprintResources/StandardMacros.DecrementInt` (`self.s`)
        (:`  `
          (`self.CalculateSML` (`self.RollWithS`) -1))))
    (elif (== _activecircle (`self.Ring_M`))
      (`SceneComponent.K2_AddLocalRotation` (`self.Ring_M`) (struct :`Yaw` 1.0) false false)
      (for _array_element_2 (`self.RollWithM`)
        (bind (_combinewith_2 _rollcount_2) (break `/Game/Blueprints/Puzzel/RotationSystem` _array_element_2))
        (bind _object_2 (`self.SetRollStruct` _combinewith_2))
        (`SceneComponent.K2_AddLocalRotation` _object_2 (`KismetMathLibrary.MakeRotator` 0.0 0.0 (`KismetMathLibrary.Conv_IntToDouble` _rollcount_2)) false false))
      (if (not (!= (`self.RollCount`) 35.0))
        (`/Engine/EditorBlueprintResources/StandardMacros.DecrementInt` (`self.m`)
          (:`  `
            (`self.CalculateSML` (`self.RollWithM`) -1))))
      (elif (== _activecircle (`self.Ring_L`))
        (`SceneComponent.K2_AddLocalRotation` (`self.Ring_L`) (struct :`Yaw` 1.0) false false)
        (for _array_element_3 (`self.RollWithL`)
          (bind (_combinewith_3 _rollcount_3) (break `/Game/Blueprints/Puzzel/RotationSystem` _array_element_3))
          (bind _object_3 (`self.SetRollStruct` _combinewith_3))
          (`SceneComponent.K2_AddLocalRotation` _object_3 (`KismetMathLibrary.MakeRotator` 0.0 0.0 (`KismetMathLibrary.Conv_IntToDouble` _rollcount_3)) false false))
        (if (not (!= (`self.RollCount`) 35.0))
          (`/Engine/EditorBlueprintResources/StandardMacros.DecrementInt` (`self.l`)
            (:`  `
              (`self.CalculateSML` (`self.RollWithL`) -1))))
        (else
          (`SceneComponent.K2_AddLocalRotation` (`self.Ring_X`) (struct :`Yaw` 1.0) false false)
          (for _array_element_4 (`self.RollWithX`)
            (bind (_combinewith_4 _rollcount_4) (break `/Game/Blueprints/Puzzel/RotationSystem` _array_element_4))
            (bind _object_4 (`self.SetRollStruct` _combinewith_4))
            (`SceneComponent.K2_AddLocalRotation` _object_4 (`KismetMathLibrary.MakeRotator` 0.0 0.0 (`KismetMathLibrary.Conv_IntToDouble` _rollcount_4)) false false))
          (if (not (!= (`self.RollCount`) 35.0))
            (`/Engine/EditorBlueprintResources/StandardMacros.DecrementInt` (`self.X`)
              (:`  `
                (`self.CalculateSML` (`self.RollWithX`) -1)))))))))

(fn `CalculateSML`
  (params (Struct :type "Array of /Game/Blueprints/Puzzel/RotationSystem Structure (by ref)") (Type :type Integer))
  (for _array_element Struct
    (bind (_combinewith _rollcount) (break `/Game/Blueprints/Puzzel/RotationSystem` _array_element))
    (if (== _combinewith (`self._s`))
      (bind _returnvalue (* _rollcount Type))
      (set `self.s` (+ (`self.s`) _returnvalue))
      (elif (== _combinewith (`self._m`))
        (set `self.m` (+ (`self.m`) _returnvalue))
        (elif (== _combinewith (`self._l`))
          (set `self.l` (+ (`self.l`) _returnvalue))
          (else
            (set `self.X` (+ (`self.X`) _returnvalue))))))))

(fn `SetActiveMaterial`
  (params (NewParam :type "StaticMeshComponent Object Reference"))
  (`PrimitiveComponent.SetMaterial` NewParam 0 "/Game/Material/puzzel/MI_QuipuPuzzle_B03.MI_QuipuPuzzle_B03"))

(fn `SetNormalMaterial`
  (params (NewParam :type "StaticMeshComponent Object Reference"))
  (`PrimitiveComponent.SetMaterial` NewParam 0 "/Game/Material/puzzel/MI_QuipuPuzzle_B02.MI_QuipuPuzzle_B02"))

(fn `SetRollStruct`
  (params (Text :type Text))
  (returns (Object :type "StaticMeshComponent Object Reference"))
  (if (== Text (`self._s`))
    (return (`self.Ring_S`))
    (elif (== Text (`self._m`))
      (return (`self.Ring_M`))
      (elif (== Text (`self._l`))
        (return (`self.Ring_L`))
        (else
          (return (`self.Ring_X`)))))))

(fn `UserConstructionScript`)