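; Old man (village chief) NPC who talks to the player and hands over the hood.
; Dialogue locks movement and steps through indexed line arrays in WB_TalkDialogue; finishing the first plays a handover animation, popup and BP_HealthCollector spawn.
; Finishing the second calls End and sets IsGetHood on GI_MyGameInstance, after which Dialogue only restores walking.
; Tick relocates him once the first memory ball is obtained; pre-ball dialogue is disconnected.
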(event `self.Talk`)

(event `self.Dialogue`
  (bind _returnvalue (`GameplayStatics.GetPlayerCharacter` 0))
  ;[1 1 1] 망토 획득 여부 체크
  (bind _asgi_my_game_instance (cast `/Game/Blueprints/GameMode/GI_MyGameInstance` (`GameplayStatics.GetGameInstance`)))
  (if (`/Game/Blueprints/GameMode/GI_MyGameInstance.bIsGetHood` _asgi_my_game_instance)
    ;[1 1 1] 망토 획득 후
    (`CharacterMovementComponent.SetMovementMode` (`Character.CharacterMovement` (`GameplayStatics.GetPlayerCharacter` 0)) "MOVE_Walking" 0)
    (else
      ;[1 1 1] 기본
      (`SceneComponent.SetVisibility` (`self.Widget`) false false)
      (`NavMovementComponent.StopActiveMovement` (`Character.CharacterMovement` (`GameplayStatics.GetPlayerCharacter` 0)))
      (`CharacterMovementComponent.DisableMovement` (`Character.CharacterMovement` (`GameplayStatics.GetPlayerCharacter` 0)))
      ;[1 1 1] 첫번째 기억구슬 획득여부 확인
      (bind _asgi_my_game_instance_2 (cast `/Game/Blueprints/GameMode/GI_MyGameInstance` (`GameplayStatics.GetGameInstance`)))
      (if (`/Game/Blueprints/GameMode/GI_MyGameInstance.bIsGetMemoryBall_First` _asgi_my_game_instance_2)
        _
        (else
          _))
      ;[1 1 1] 기억구슬 획득 후
      (if (== 1 (`self.dialogueIndex`))
        ;;[0.3325 0.3325 0.3325] 1번 대화 - 대화 추가하고 싶으시면 이거 복사해서 숫자 달려있는 변수들 변경해서 쓰십셔
        (`/Engine/EditorBlueprintResources/StandardMacros.IncrementInt` (`self.TalkIndex`)
          (:`  `
            (if (< (`self.TalkIndex`) (`KismetArrayLibrary.Array_Length` (`self.newDialogue1`)))
              (`self.UI`
                (:`then`
                  _)
                (:`else`
                  (bind _returnvalue_2 (`|CreateWidget` "/Game/Blueprints/Dialogue/WB_TalkDialogue.WB_TalkDialogue_C" (`GameplayStatics.GetPlayerController` 0)))
                  (bind _output_get (set `self.UI` _returnvalue_2))
                  (`UserWidget.AddToViewport` _output_get 0)))
              (`TextBlock.SetText` (`/Game/Blueprints/Dialogue/WB_TalkDialogue.DialogueText` (`self.UI`)) (`KismetTextLibrary.Conv_StringToText` (`|GetArrayItem` (`self.newDialogue1`) (`self.TalkIndex`))))
              (`GameplayStatics.PlaySound2D` (`self.Sound_1`) 1.0 1.0 0.0 null null)
              (else
                (set `self.TalkIndex` -1)
                (set `self.dialogueIndex` 0)
                (`self.DisableInput` null)
                ;[1 1 1] 건내는 애니메이샨
                (`SkeletalMeshComponent.PlayAnimation` (`self.Mesh`) "/Game/Characters/OldWoman/Animation/Oldwoman_Talking.Oldwoman_Talking" false)
                (`KismetSystemLibrary.Delay` 2.0)
                ;[0.1947 1 0] 여기에 위젯 삽입
                (bind _returnvalue_3 (`|CreateWidget` "/Game/Blueprints/UI/WB_ItemPopup.WB_ItemPopup_C"))
                (bind _output_get_2 (set `self.PopupWidgetRef` _returnvalue_3))
                (`UserWidget.AddToViewport` _output_get_2 0)
                (`KismetSystemLibrary.Delay` 5.0)
                (`Widget.RemoveFromParent` (`self.PopupWidgetRef`))
                ;[1 1 1] 망토 건내기
                (`|SpawnActorFromClass` "/Game/Blueprints/BP_HealthCollector.BP_HealthCollector_C" (`self.GetTransform` _returnvalue) "Undefined" "MultiplyWithRoot" null null)
                (`self.EnableInput` _returnvalue null)
                (if (== 2 (`self.dialogueIndex`)) :!label _label
                  ;;[0.3325 0.3325 0.3325] 2번 대화
                  (`/Engine/EditorBlueprintResources/StandardMacros.IncrementInt` (`self.TalkIndex`)
                    (:`  `
                      (if (< (`self.TalkIndex`) (`KismetArrayLibrary.Array_Length` (`self.newDialogue2`)))
                        (`self.UI`
                          (:`then`
                            _)
                          (:`else`
                            (bind _returnvalue_4 (`|CreateWidget` "/Game/Blueprints/Dialogue/WB_TalkDialogue.WB_TalkDialogue_C" (`GameplayStatics.GetPlayerController` 0)))
                            (bind _output_get_3 (set `self.UI` _returnvalue_4))
                            (`UserWidget.AddToViewport` _output_get_3 0)))
                        (`TextBlock.SetText` (`/Game/Blueprints/Dialogue/WB_TalkDialogue.DialogueText` (`self.UI`)) (`KismetTextLibrary.Conv_StringToText` (`|GetArrayItem` (`self.newDialogue2`) (`self.TalkIndex`))))
                        (`GameplayStatics.PlaySound2D` (`self.Sound_2`) 1.0 1.0 0.0 null null)
                        (`self.DestoryDon'tPass`)
                        (else
                          (`self.End`)
                          (bind _asgi_my_game_instance_3 (cast `/Game/Blueprints/GameMode/GI_MyGameInstance` (`GameplayStatics.GetGameInstance`)))
                          (set `/Game/Blueprints/GameMode/GI_MyGameInstance.bIsGetHood` true _asgi_my_game_instance_3))))))))))
        (else
          (goto _label))))))

(event `self.ReceiveTick`
  (params (DeltaSeconds :type "Float (single-precision)"))
  ;[1 1 1] 기억구슬 획득시 이장 로케이션 변경
  (bind _asgi_my_game_instance (cast `/Game/Blueprints/GameMode/GI_MyGameInstance` (`GameplayStatics.GetGameInstance`)))
  (if (`/Game/Blueprints/GameMode/GI_MyGameInstance.bIsGetMemoryBall_First` _asgi_my_game_instance)
    (`self.ChangeLocation`)
    (`self.DestoryLocationLight`)))

(event `EnhancedInput|/Game/Blueprints/Input/IA_Interact`
  (params (ActionValue :type Boolean) (ElapsedSeconds :type "Float (double-precision)") (TriggeredSeconds :type "Float (double-precision)") (InputAction :type "InputAction Object Reference" :default "/Game/Blueprints/Input/IA_Interact.IA_Interact"))
  (:`Started`
    (`KismetSystemLibrary.PrintString` "Hello")))

(event `InputAction|IA_Interact`
  (params (Key :type "Key Structure")))

(fn `ChangeLocation`
  (`self.K2_SetActorLocationAndRotation` (9290.844397 -2341.887013 1193.58658) (struct :`Yaw` -145.758996)))

(fn `End`
  ;[1 1 1] 대화 종료
  (`Widget.RemoveFromParent` (`self.UI`))
  (`SceneComponent.SetVisibility` (`self.Widget`) true false)
  (`CharacterMovementComponent.SetMovementMode` (`Character.CharacterMovement` (`GameplayStatics.GetPlayerCharacter` 0)) "MOVE_Walking" 0)
  (set `self.TalkIndex` -1)
  (set `self.UI` null)
  (if (== (`self.dialogueCount`) (`self.dialogueIndex`))
    (set `self.dialogueIndex` 1) ; 첫 번째 대화로 초기화
    (else
      (`/Engine/EditorBlueprintResources/StandardMacros.IncrementInt` (`self.dialogueIndex`)))))

(fn `Remove popup`
  (`Widget.RemoveFromParent` (`self.PopupWidgetRef`)))

(fn `UserConstructionScript`
  (`parent.UserConstructionScript`))