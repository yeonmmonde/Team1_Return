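; BP_MemoryPaPer_A01 is a pickup for memory paper A01 that triggers when BP_Maincharacter overlaps its box.
; On overlap it reveals the MemoryPaperA01 entry in the character's pause menu, disables player movement and flags the paper as obtained in GI_MyGameInstance.
; It then plays a pickup sound, destroys itself and opens the WB_PaperA01ZoomIn widget.
; Nothing in this Blueprint re-enables movement.
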(event `self.Box.OnComponentBeginOverlap`
  (params (OverlappedComponent :type "PrimitiveComponent Object Reference") (OtherActor :type "Actor Object Reference") (OtherComp :type "PrimitiveComponent Object Reference") (OtherBodyIndex :type Integer) (bFromSweep :type Boolean) (SweepResult :type "HitResult Structure (by ref)"))
  (bind _asbp_maincharacter (cast `/Game/Blueprints/BP_Maincharacter` OtherActor))
  (`Widget.SetVisibility` (`/Game/Blueprints/UI/WB_PauseMenu.MemoryPaper_A01` (`/Game/Blueprints/BP_Maincharacter.Pause Menu Widget` _asbp_maincharacter)) "SelfHitTestInvisible")
  (`NavMovementComponent.StopActiveMovement` (`Character.CharacterMovement` (`GameplayStatics.GetPlayerCharacter` 0)))
  (`CharacterMovementComponent.DisableMovement` (`Character.CharacterMovement` (`GameplayStatics.GetPlayerCharacter` 0)))
  (bind _asgi_my_game_instance (cast `/Game/Blueprints/GameMode/GI_MyGameInstance` (`GameplayStatics.GetGameInstance`)))
  (set `/Game/Blueprints/GameMode/GI_MyGameInstance.bIsGetPaperA01` true _asgi_my_game_instance)
  (`GameplayStatics.PlaySound2D` "/Game/Audio/ItemPickup/Paper_Pickup.Paper_Pickup" 1.0 1.0 0.0 null null)
  (`self.K2_DestroyActor`)
  (bind _returnvalue (`|CreateWidget` "/Game/Blueprints/UI/WB_PaperA01ZoomIn.WB_PaperA01ZoomIn_C"))
  (`UserWidget.AddToViewport` _returnvalue 0))

(fn `UserConstructionScript`)