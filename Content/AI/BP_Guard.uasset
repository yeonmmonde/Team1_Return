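; BP_Guard is an enemy guard for a stealth game that can catch the player and be taken down.
; An overlap radius shows a takedown prompt to the player while the guard is alive, and a takedown event ragdolls it after a short delay.
; Run raises walk speed, while Catch plays a montage whose notify sphere-traces ahead and reports a player hit once to the stealth game mode as a capture.
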(event `Takedown Ragdoll`
  (`KismetSystemLibrary.Delay` 1.27)
  (`PrimitiveComponent.SetSimulatePhysics` (`self.Mesh`) true)
  (`CharacterMovementComponent.SetMovementMode` (`self.CharacterMovement`) "MOVE_None" 0))

(event `self.Takedown Radius.OnComponentBeginOverlap`
  (params (OverlappedComponent :type "PrimitiveComponent Object Reference") (OtherActor :type "Actor Object Reference") (OtherComp :type "PrimitiveComponent Object Reference") (OtherBodyIndex :type Integer) (bFromSweep :type Boolean) (SweepResult :type "HitResult Structure (by ref)"))
  (if (and (`self.ActorHasTag` OtherActor "Player") (not (`self.dead`)))
    (`SceneComponent.SetVisibility` (`self.Takedown Prompt Widget`) true false)))

(event `self.Takedown Radius.OnComponentEndOverlap`
  (params (OverlappedComponent :type "PrimitiveComponent Object Reference") (OtherActor :type "Actor Object Reference") (OtherComp :type "PrimitiveComponent Object Reference") (OtherBodyIndex :type Integer))
  (if (`self.ActorHasTag` OtherActor "Player")
    (`SceneComponent.SetVisibility` (`self.Takedown Prompt Widget`) false false)))

(event `Run_1`
  (set `CharacterMovementComponent.MaxWalkSpeed` 500.0 (`self.CharacterMovement`)))

(event `Catch_1`
  (bind _returnvalue (`self.K2_GetActorLocation`))
  (if (not (`self.is attacking`))
    (`|PlayMontage` (`self.Mesh`) "/Game/Characters/Robber/Catch/Catch_Montage.Catch_Montage"
      (:`then`
        (set `self.is attacking` true))
      (:`OnCompleted`
        (set `self.is attacking` false))
      (:`OnNotifyBegin`
        (bind (_outhit _returnvalue_2) (`KismetSystemLibrary.SphereTraceSingleForObjects` :`Start` _returnvalue :`End` (+ _returnvalue (* (`self.GetActorForwardVector`) 125.0)) :`Radius` 30.0 :`ObjectTypes` (`|MakeArray` "ObjectTypeQuery3" :!type "EObjectTypeQuery Enum") :`DrawDebugType` "ForDuration"))
        (if _returnvalue_2
          (if (`self.ActorHasTag` (`.HitActor` (`GameplayStatics.BreakHitResult` _outhit)) "Player")
            (`/Engine/EditorBlueprintResources/StandardMacros.DoOnce` false
              (:`Completed`
                (bind _asgm_stealth_game_mode (cast `/Game/Blueprints/GameMode/GM_StealthGameMode` (`GameplayStatics.GetGameMode`)))
                (`/Game/Blueprints/GameMode/GM_StealthGameMode.Captured` _asgm_stealth_game_mode)))))))))

(fn `UserConstructionScript`)