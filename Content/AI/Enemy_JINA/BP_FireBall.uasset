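; BP_FireBall is an enemy fireball actor that flies toward the spot where the player stood when it spawned.
; BeginPlay caches the location of player 0's character, and Tick steps toward that fixed point at Speed, scaled by delta time, so it does not home.
; Movement is an unswept SetActorLocation, and the graph has no arrival check, damage or destroy logic.
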(event `self.ReceiveBeginPlay`
  (set `self.location` (`self.K2_GetActorLocation` (`GameplayStatics.GetPlayerCharacter` 0))))

(event `self.ReceiveTick`
  (params (DeltaSeconds :type "Float (single-precision)"))
  (bind _returnvalue (`self.K2_GetActorLocation`))
  (`self.K2_SetActorLocation` (+ _returnvalue (* (`KismetMathLibrary.Normal` (- (`self.location`) _returnvalue)) (`self.speed`) DeltaSeconds))))

(fn `UserConstructionScript`)