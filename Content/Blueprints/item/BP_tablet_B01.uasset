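; Pickup actor for tablet piece B, described in its popup as the Quipu Puzzle reward.
; Box overlap by the main character sets the tablet flags on GameInstance and character, reveals its pause-menu slot, and stops movement.
; It plays a sound, calls DestroyActor, then still builds and shows the item popup.
; The Interact handler on this same actor closes the popup and restores walking.
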(event `self.Box.OnComponentBeginOverlap`
  (params (OverlappedComponent :type "PrimitiveComponent Object Reference") (OtherActor :type "Actor Object Reference") (OtherComp :type "PrimitiveComponent Object Reference") (OtherBodyIndex :type Integer) (bFromSweep :type Boolean) (SweepResult :type "HitResult Structure (by ref)"))
  (bind _asbp_maincharacter (cast `/Game/Blueprints/BP_Maincharacter` OtherActor))
  (bind _asgi_my_game_instance (cast `/Game/Blueprints/GameMode/GI_MyGameInstance` (`GameplayStatics.GetGameInstance`)))
  (set `/Game/Blueprints/GameMode/GI_MyGameInstance.HasTabletB` true _asgi_my_game_instance)
  (set `/Game/Blueprints/BP_Maincharacter.has tablet2` true _asbp_maincharacter)
  (bind _pause_menu_widget (`/Game/Blueprints/BP_Maincharacter.Pause Menu Widget` _asbp_maincharacter))
  (`Widget.SetIsEnabled` (`/Game/Blueprints/UI/WB_PauseMenu.slot2` _pause_menu_widget) true)
  (`Widget.SetVisibility` (`/Game/Blueprints/UI/WB_PauseMenu.TN_tableet_B01` _pause_menu_widget) "SelfHitTestInvisible")
  (`GameplayStatics.GetActorOfClass` "/Game/Blueprints/item/door/BP_OpenDoor.BP_OpenDoor_C")
  (`self.DisableInput` null)
  (`NavMovementComponent.StopActiveMovement` (`Character.CharacterMovement` (`GameplayStatics.GetPlayerCharacter` 0)))
  (`CharacterMovementComponent.DisableMovement` (`Character.CharacterMovement` (`GameplayStatics.GetPlayerCharacter` 0)))
  (`GameplayStatics.PlaySound2D` "/Game/Audio/Effect/itempicksound.itempicksound" 1.0 1.0 0.0 null null)
  (`KismetSystemLibrary.PrintText` "You got the tablet1")
  (`self.K2_DestroyActor`)
  ;[1 1 1] Item Popup\
  (bind _returnvalue (`|CreateWidget` "/Game/Blueprints/UI/WB_ItemPopup.WB_ItemPopup_C" (`GameplayStatics.GetPlayerController` 0)))
  (bind _output_get (set `self.PopupWidgetRef` _returnvalue))
  (`Image.SetBrush` (`/Game/Blueprints/UI/WB_ItemPopup.ItemImage` _output_get) (make `SlateBrush` "Image" "NoTile" "NoMirror" (struct :`X` 32.0 :`Y` 32.0) (struct) (struct :`SpecifiedColor` (struct :`R` 1.0 :`G` 1.0 :`B` 1.0 :`A` 1.0) :`ColorUseRule` "UseColor_Specified") (struct :`CornerRadii` (struct :`W` 1.0) :`Color` (struct :`SpecifiedColor` (struct) :`ColorUseRule` "UseColor_Specified") :`RoundingType` "HalfHeightRadius") "/Game/Modeling/item/TN_Tablet_B01.TN_Tablet_B01"))
  (`TextBlock.SetText` (`/Game/Blueprints/UI/WB_ItemPopup.ItemName` _output_get) "Broken piece of stone tablet (B)")
  (`TextBlock.SetText` (`/Game/Blueprints/UI/WB_ItemPopup.ItemInformation` _output_get) "The remaining pieces of the tablet that came out after solving the Quipu Puzzle. It looks like the two tablets can be combined together and be used somewhere. ")
  (`UserWidget.AddToViewport` _output_get 0)
  (`self.EnableInput` (`GameplayStatics.GetPlayerCharacter` 0) (`GameplayStatics.GetPlayerController` 0))
  (set `self.IsItemWidgetOn` true))

(event `InputAction|IA_Interact`
  (params (Key :type "Key Structure"))
  (:`Pressed`
    (if (`self.IsItemWidgetOn`)
      (`Widget.RemoveFromParent` (`self.PopupWidgetRef`))
      (set `self.IsItemWidgetOn` false)
      (`CharacterMovementComponent.SetMovementMode` (`Character.CharacterMovement` (`GameplayStatics.GetPlayerCharacter` 0)) "MOVE_Walking" 0))))

(fn `UserConstructionScript`)