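; Sun God NPC dialogue Blueprint that gives the player the Heart of Pachamama.
; Each Dialogue event locks movement and advances one line, choosing between two pre-gift sets and a post-gift set via GameInstance.HasHeart.
; After the first set, a giving animation leads to an item popup; DeleteWidget closes it, spawns the heart and starts the second set, whose end sets HasHeart.
; BeginPlay swaps only the post-gift lines to Korean when IsKorean is set.
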(event `/Game/Blueprints/Dialogue/BPI_Dialogue.Dialogue`
  ;[1 1 1] 기본
  (`SceneComponent.SetVisibility` (`self.Widget`) false false)
  (`NavMovementComponent.StopActiveMovement` (`Character.CharacterMovement` (`GameplayStatics.GetPlayerCharacter` 0)))
  (`CharacterMovementComponent.DisableMovement` (`Character.CharacterMovement` (`GameplayStatics.GetPlayerCharacter` 0)))
  ;[1 1 1] 아이템 획득 여부 체크
  (if (`/Game/Blueprints/GameMode/GI_MyGameInstance.HasHeart` (`self._GameInstance`))
    ;[1 1 1] AfterGetHood
    ;;[0.3325 0.3325 0.3325] 1번 대화 - 대화 추가하고 싶으시면 이거 복사해서 숫자 달려있는 변수들 변경해서 쓰십셔
    (`/Engine/EditorBlueprintResources/StandardMacros.IncrementInt` (`self.TalkIndex`)
      (:`  `
        (if (< (`self.TalkIndex`) (`KismetArrayLibrary.Array_Length` (`self.AfterGetItemDialogue1`)))
          (`self.UI`
            (:`then`
              _)
            (:`else`
              (bind _returnvalue (`|CreateWidget` "/Game/Blueprints/Dialogue/WB_TalkDialogue.WB_TalkDialogue_C" (`GameplayStatics.GetPlayerController` 0)))
              (bind _output_get (set `self.UI` _returnvalue))
              (`UserWidget.AddToViewport` _output_get 0)))
          (`TextBlock.SetText` (`/Game/Blueprints/Dialogue/WB_TalkDialogue.DialogueText` (`self.UI`)) (`KismetTextLibrary.Conv_StringToText` (`|GetArrayItem` (`self.AfterGetItemDialogue1`) (`self.TalkIndex`))))
          (`GameplayStatics.PlaySound2D` (`self.Sound_1`) 1.0 1.0 0.0 null null)
          (else
            (`self.EndDialogue`)))))
    (else
      ;[1 1 1] Before Get Heart
      (if (== 1 (`self.dialogueIndex`))
        ;;[0.3325 0.3325 0.3325] 1번 대화 - 대화 추가하고 싶으시면 이거 복사해서 숫자 달려있는 변수들 변경해서 쓰십셔
        (`/Engine/EditorBlueprintResources/StandardMacros.IncrementInt` (`self.TalkIndex`)
          (:`  `
            (if (< (`self.TalkIndex`) (`KismetArrayLibrary.Array_Length` (`self.dialogue1`)))
              (`self.UI`
                (:`then`
                  _)
                (:`else`
                  (bind _returnvalue_2 (`|CreateWidget` "/Game/Blueprints/Dialogue/WB_TalkDialogue.WB_TalkDialogue_C" (`GameplayStatics.GetPlayerController` 0)))
                  (bind _output_get_2 (set `self.UI` _returnvalue_2))
                  (`UserWidget.AddToViewport` _output_get_2 0)))
              (`TextBlock.SetText` (`/Game/Blueprints/Dialogue/WB_TalkDialogue.DialogueText` (`self.UI`)) (`KismetTextLibrary.Conv_StringToText` (`|GetArrayItem` (`self.dialogue1`) (`self.TalkIndex`))))
              (`GameplayStatics.PlaySound2D` (`self.Sound_1`) 1.0 1.0 0.0 null null)
              (else
                (set `self.TalkIndex` -1)
                (set `self.dialogueIndex` 2)
                (`self.DisableInput` (`GameplayStatics.GetPlayerCharacter` 0) (`GameplayStatics.GetPlayerController` 0))
                ;[1 1 1] 건내는 애니메이샨
                (`SkeletalMeshComponent.PlayAnimation` (`self.Mesh`) "/Game/Characters/SunGod/Animation/SunGod_Sitting_And_Giving.SunGod_Sitting_And_Giving" false)
                (`KismetSystemLibrary.Delay` 2.0)
                ;[0.1947 1 0] 여기에 위젯 삽입
                (bind _returnvalue_3 (`|CreateWidget` "/Game/Blueprints/UI/WB_ItemPopup.WB_ItemPopup_C" (`GameplayStatics.GetPlayerController` 0)))
                (bind _output_get_3 (set `self.PopupWidgetRef` _returnvalue_3))
                (`Image.SetBrush` (`/Game/Blueprints/UI/WB_ItemPopup.ItemImage` _output_get_3) (make `SlateBrush` "Image" "NoTile" "NoMirror" (struct :`X` 32.0 :`Y` 32.0) (struct) (struct :`SpecifiedColor` (struct :`R` 1.0 :`G` 1.0 :`B` 1.0 :`A` 1.0) :`ColorUseRule` "UseColor_Specified") (struct :`CornerRadii` (struct :`W` 1.0) :`Color` (struct :`SpecifiedColor` (struct) :`ColorUseRule` "UseColor_Specified") :`RoundingType` "HalfHeightRadius") "/Game/Modeling/item/TN_BrokenHeart_A01.TN_BrokenHeart_A01"))
                (`TextBlock.SetText` (`/Game/Blueprints/UI/WB_ItemPopup.ItemName` _output_get_3) "The Heart of Pachamama")
                (`TextBlock.SetText` (`/Game/Blueprints/UI/WB_ItemPopup.ItemInformation` _output_get_3) "A crystal that contains Pachamama's power. Kaira says that Pachamama's power will return when Heart is placed at the Altar of Healing at the top of the tree.")
                (`UserWidget.AddToViewport` _output_get_3 0)
                (`self.EnableInput` (`GameplayStatics.GetPlayerCharacter` 0) (`GameplayStatics.GetPlayerController` 0))
                (set `self.IsItemWidgetOn` true)))))
        (elif (== 2 (`self.dialogueIndex`))
          ;;[0.3325 0.3325 0.3325] 2번 대화
          (`/Engine/EditorBlueprintResources/StandardMacros.IncrementInt` (`self.TalkIndex`) :!label _label
            (:`  `
              (if (< (`self.TalkIndex`) (`KismetArrayLibrary.Array_Length` (`self.dialogue2`)))
                (`self.UI`
                  (:`then`
                    _)
                  (:`else`
                    (bind _returnvalue_4 (`|CreateWidget` "/Game/Blueprints/Dialogue/WB_TalkDialogue.WB_TalkDialogue_C" (`GameplayStatics.GetPlayerController` 0)))
                    (bind _output_get_4 (set `self.UI` _returnvalue_4))
                    (`UserWidget.AddToViewport` _output_get_4 0)))
                (`TextBlock.SetText` (`/Game/Blueprints/Dialogue/WB_TalkDialogue.DialogueText` (`self.UI`)) (`KismetTextLibrary.Conv_StringToText` (`|GetArrayItem` (`self.dialogue2`) (`self.TalkIndex`))))
                (`GameplayStatics.PlaySound2D` (`self.Sound_2`) 1.0 1.0 0.0 null null)
                (else
                  (`self.EndDialogue`)
                  (set `/Game/Blueprints/GameMode/GI_MyGameInstance.HasHeart` true (`self._GameInstance`)))))))))))

(event `self.ReceiveBeginPlay`
  (bind _asgi_my_game_instance (cast `/Game/Blueprints/GameMode/GI_MyGameInstance` (`GameplayStatics.GetGameInstance`)))
  (bind _output_get (set `self._GameInstance` _asgi_my_game_instance))
  (if (`/Game/Blueprints/GameMode/GI_MyGameInstance.bIsKorean` _output_get)
    (set `self.AfterGetItemDialogue1` (`self.K_AfterGetItemDialogue1`))))

(event `/Game/Blueprints/UI/BPI_DeleteWidget.DeleteWidget`
  (`Widget.RemoveFromParent` (`self.PopupWidgetRef`))
  ;[1 1 1] Give Item
  (`|SpawnActorFromClass` "/Game/Blueprints/item/BP_BrokenHeart_A01.BP_BrokenHeart_A01_C" (`self.GetTransform` (`GameplayStatics.GetPlayerCharacter` 0)) "Undefined" "MultiplyWithRoot" null null)
  (goto _label))

(fn `UserConstructionScript`
  (`parent.UserConstructionScript`))