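; Game mode for the main character that handles player spawning, the captured state and escape music.
; New players start at the PlayerStart named by the options string minus its first character.
; SwitchMusictoEscaping fades out Music and starts the escape track; Captured shows the cursor and fading capture widget, stopping that track with a caught sound if valid.
; BeginPlay is empty, and the music and rain startup chain is disconnected, so Music is never assigned here.
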(event `self.ReceiveBeginPlay`)

(event `Captured`
  (bind _returnvalue (`GameplayStatics.GetPlayerController` 0))
  (set `PlayerController.bShowMouseCursor` true _returnvalue)
  (`WidgetBlueprintLibrary.SetInputMode_GameAndUIEx` _returnvalue null)
  (bind _returnvalue_2 (`|CreateWidget` "/Game/Blueprints/UI/WB_Captured.WB_Captured_C"))
  (bind _output_get (set `self.Captured Widget` _returnvalue_2))
  (`UserWidget.AddToViewport` _output_get 0)
  (`/Game/Blueprints/UI/WB_Captured.Play Fade Animation` (`self.Captured Widget`))
  (bind _escaping_music (`self.Escaping Music`)
    (:`then`
      (`AudioComponent.FadeOut` _escaping_music 0.3 0.0 "Linear")
      (`GameplayStatics.PlaySound2D` "/Game/Audio/Effect/Caught.Caught" 1.0 1.0 0.0 null null))
    (:`else`)))

(event `Switch Music to Escaping`
  (`AudioComponent.FadeOut` (`self.Music`) 0.3 0.0 "Linear")
  (bind _returnvalue (`GameplayStatics.SpawnSound2D` "/Game/Audio/Music/Escaping.Escaping" 0.5 1.0 0.0 null))
  (set `self.Escaping Music` _returnvalue))

(event `self.HandleStartingNewPlayer`
  (params (NewPlayer :type "PlayerController Object Reference"))
  (bind _optionsstring (`self.OptionsString`))
  ;[1 1 1] PlayerLocation
  (`self.RestartPlayerAtPlayerStart` NewPlayer (`self.K2_FindPlayerStart` NewPlayer (`KismetStringLibrary.GetSubstring` _optionsstring 1 (- (`KismetStringLibrary.Len` _optionsstring) 1)))))

(fn `UserConstructionScript`)