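; Rotating alarm sensor that detects the robber player after they linger in its detection zone.
; A ping-ponging timeline sweeps the head back and forth while the zone's overlap events start and stop a fast looping timer.
; The timer fills the player's detection meter, calling DetectPlayer and flagging the widget as detected at the threshold.
; Leaving the zone resets the count, and clears the meter unless already detected.
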(event `self.ReceiveBeginPlay`
  (`|ExecutionSequence`
    (:`then_0`
      (bind (_direction _rotation) (`Timeline|Motion` :!label _label)
        (:`Update`
          (`SceneComponent.K2_SetRelativeRotation` (`self.Head`) (`KismetMathLibrary.RLerp` (struct :`Yaw` 90.0) (struct :`Yaw` -90.0) _rotation) false false))
        (:`Finished`
          (`/Engine/EditorBlueprintResources/StandardMacros.FlipFlop`
            (:`A`
              (goto _label :!via `Reverse`))
            (:`B`
              (goto _label))))))
    (:`then_1`
      (bind _asbp_robber (cast `/Game/Blueprints/BP_Robber` (`GameplayStatics.GetPlayerCharacter` 0)))
      (set `self.Player BP` _asbp_robber))))

(event `self.Trigger Detection Zone.OnComponentBeginOverlap`
  (params (OverlappedComponent :type "PrimitiveComponent Object Reference") (OtherActor :type "Actor Object Reference") (OtherComp :type "PrimitiveComponent Object Reference") (OtherBodyIndex :type Integer) (bFromSweep :type Boolean) (SweepResult :type "HitResult Structure (by ref)"))
  (if (`self.ActorHasTag` OtherActor "Player")
    (set `self.player in zone` true)
    (bind _returnvalue (`KismetSystemLibrary.K2_SetTimerDelegate` (delegate `Count`) 0.002 true))
    (set `self.Count TImer` _returnvalue)))

(event `Count`
  (set `self.time under zone` (+ (`self.time under zone`) 0.005))
  (`self.Update Progress Bar`)
  (if (>= (`self.time under zone`) 3.0)
    (`self.Detect Player` (stale `self.Trigger Detection Zone.OnComponentBeginOverlap` OtherActor))
    (`KismetSystemLibrary.K2_ClearAndInvalidateTimerHandle` (`self.Count TImer`))
    (`/Game/UI/WB_DetectionMeter.Detected` (`/Game/Blueprints/BP_Robber.Detected Meter Widget` (`self.Player BP`)))))

(event `Update Progress Bar`
  (bind _detected_meter_widget (`/Game/Blueprints/BP_Robber.Detected Meter Widget` (`self.Player BP`)))
  (if (not (`/Game/UI/WB_DetectionMeter.detected?` _detected_meter_widget))
    (`ProgressBar.SetPercent` (`/Game/UI/WB_DetectionMeter.ProgressBar` _detected_meter_widget) (/ (`self.time under zone`) 3.0))))

(event `self.Trigger Detection Zone.OnComponentEndOverlap`
  (params (OverlappedComponent :type "PrimitiveComponent Object Reference") (OtherActor :type "Actor Object Reference") (OtherComp :type "PrimitiveComponent Object Reference") (OtherBodyIndex :type Integer))
  (bind _detected_meter_widget (`/Game/Blueprints/BP_Robber.Detected Meter Widget` (`self.Player BP`)))
  (if (`self.ActorHasTag` OtherActor "Player")
    (set `self.player in zone` false)
    (`KismetSystemLibrary.K2_ClearAndInvalidateTimerHandle` (`self.Count TImer`))
    (set `self.time under zone` 0.0)
    (if (not (`/Game/UI/WB_DetectionMeter.detected?` _detected_meter_widget))
      (`ProgressBar.SetPercent` (`/Game/UI/WB_DetectionMeter.ProgressBar` _detected_meter_widget) 0.0))))

(fn `UserConstructionScript`
  (`parent.UserConstructionScript`))